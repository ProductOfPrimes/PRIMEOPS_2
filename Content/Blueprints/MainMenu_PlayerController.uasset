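; Main menu player controller that lets each local player choose and confirm a mech slot.
; D-Pad left and right presses send the player's controller ID and key to the main menu HUD to update that player's slot.
; Confirm and Cancel inputs confirm or cancel that slot through the same HUD.
; The HUD reference is supplied through an Init function.
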(event EventBeginPlay)

(event EventTick
  (params (DeltaSeconds :type Float%20%28single-precision%29)))

(event Input|ActionEvents|InputActionD-PadRight
  (params (Key :type Key%20Structure :default "None"))
  (:Pressed
    (Default|UpdateControllerPlayerSlot (Variables|Default|GetMainMenuHUD) (Class|GameplayStatics|GetPlayerControllerID self) Key)))

(event Input|ActionEvents|InputActionD-PadLeft
  (params (Key :type Key%20Structure :default "None"))
  (:Pressed
    (Default|UpdateControllerPlayerSlot (Variables|Default|GetMainMenuHUD) (Class|GameplayStatics|GetPlayerControllerID self) Key)))

(event Input|ActionEvents|InputActionConfirm
  (params (Key :type Key%20Structure :default "None"))
  (:Pressed
    (Default|ConfirmMechSlot (Variables|Default|GetMainMenuHUD) (Class|GameplayStatics|GetPlayerControllerID self))))

(event Input|ActionEvents|InputActionCancel
  (params (Key :type Key%20Structure :default "None"))
  (:Pressed
    (Default|CancelMechSlot (Variables|Default|GetMainMenuHUD) (Class|GameplayStatics|GetPlayerControllerID self))))

(fn ConstructionScript)

(fn Init
  (params (hud :type HUD%20Main%20Menu%20Object%20Reference%20%28by%20ref%29))
  (Variables|Default|SetMainMenuHUD hud))