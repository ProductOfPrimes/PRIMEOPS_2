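; Game state for team deathmatch (TDM) that tracks when mechs are ready and starts the battle.
; Collects mechs as they report ready, enabling each, until their count matches PlayerArray, then sets BattleReadyState and passes the list on through OnAllMechsReady.
; Ready-state changes, including an OnRep handler, show "READY?" or "GO!!!!!" on the HUD, and a helper refreshes player cooldown cards.
; Mech spawning and loadout code is present but disconnected.
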(event Custom|EventOnMechReady
  (params (Mech :type Mech%20Pawn%20Object%20Reference))
  (CallFunction|MechReadyServer Mech))

(event Custom|Mech%20Ready%20Server
  (params (Mech :type Mech%20Pawn%20Object%20Reference))
  (bind _mechs (Variables|Default|GetMechs))
  (Utilities|Array|AddUnique _mechs Mech)
  (Variables|/Game/Blueprints/Mech_Pawn.Mech_Pawn_C|SetCanAct Mech true)
  (if (== (Utilities|Array|Length _mechs) (Utilities|Array|Length (Variables|Default|GetPlayerArray)))
    (CallFunction|EventonAllMechsReadyServer)))

(event Custom|EventOnAllMechsReadyClient
  (params (Mechs :type Array%20of%20Mech%20Pawn%20Object%20References))
  (bind _output_get (Variables|Default|SetMechs Mechs))
  (Default|CallOnAllMechsReady _output_get))

(event Custom|EventOnAllMechsReadyServer
  (Variables|Default|SetBattleReadyState 1)
  (CallFunction|UpdateBasedonReadyState)
  (bind _array_element (Utilities|Array|ForEachLoopwithBreak (Variables|Default|GetMechs))
    (:LoopBody
      (Variables|/Game/Blueprints/Mech_Pawn.Mech_Pawn_C|SetCanAct _array_element true))
    (:Completed
      (CallFunction|EventonAllMechsReadyClient (Variables|Default|GetMechs)))))

(event EventBeginPlay
  (EventDispatchers|BindEventtoOnMechReady (delegate Custom|EventOnMechReady))
  (Utilities|FlowControl|Delay 0.2)
  (Variables|Default|SetBattleReadyState 0)
  (CallFunction|UpdateBasedonReadyState))

(event EventTick
  (params (DeltaSeconds :type Float%20%28single-precision%29)))

(fn ConstructionScript)

(fn OnRepReadyState
  (CallFunction|UpdateBasedonReadyState))

(fn UpdateBasedonReadyState
  (bind _asgame_hud (Utilities|Casting|CastToGameHUD (HUD|GetHUD (Game|GetPlayerController 0))))
  (Default|DisplayOnscreenMessage _asgame_hud (Utilities|Select :Index (Variables|Default|GetBattleReadyState) :Option%200 "READY?" :Option%201 "GO!!!!!") 4.0))

(fn UpdatePlayerCards
  (bind _asgame_hud (Utilities|Casting|CastToGameHUD (HUD|GetHUD (Game|GetPlayerController 0))))
  (bind _asplayer_cooldowns_ui (Utilities|Casting|CastToPlayerCooldownsUI (UserInterface|GetUserWidgetObject (Variables|/Game/UI/Gameplay/GameHUD.GameHUD_C|GetCooldownHUD _asgame_hud))))
  (Default|UpdatePlayerCards _asplayer_cooldowns_ui))