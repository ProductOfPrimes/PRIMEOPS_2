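; LivingActorComponent is an actor component that gives its owner health, an alive state and a team.
; Health starts at maximum on BeginPlay, and TakeDamage subtracts from it while alive, reporting whether that hit killed the owner.
; On reaching zero it clears the alive flag and calls OnDeath, which only prints a death message with owner name and team.
; GetHealthPercent exposes health as a fraction of maximum.
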(event EventBeginPlay
  (Variables|Default|SetCurrentHealth (Variables|Default|GetMaxHealth)))

(event EventTick
  (params (DeltaSeconds :type Float%20%28single-precision%29)))

(fn TakeDamage
  (params (DamageAmount :type Float%20%28single-precision%29))
  (if (Variables|Default|GetisAlive)
    (bind _output_get (Variables|Default|SetCurrentHealth (- (Variables|Default|GetCurrentHealth) DamageAmount)))
    (if (<= _output_get 0.0)
      (Variables|Default|SetisAlive false)
      (CallFunction|OnDeath)
      (return (<= _output_get 0.0)))
    (else
      (return false))))

(fn OnDeath
  (Development|PrintString (Utilities|String|BuildString(Name) (Utilities|GetDisplayName (Components|GetOwner)) " on team " (Utilities|Name|EnumtoName (Variables|Default|GetTeam)) "Died") true true "(R=0.980592,G=0.000000,B=1.000000,A=1.000000)"))

(fn GetHealthPercent
  (return (/ (Variables|Default|GetCurrentHealth) (Variables|Default|GetMaxHealth))))