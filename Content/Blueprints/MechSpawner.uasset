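; MechSpawner is a placed actor that spawns a player's mech at its own transform when play begins, on the server only.
; It looks up its configured player ID in MadMechsGameInstance and, if that slot is filled, reads the loadout, team and slot.
; It spawns a Mech_Pawn with that slot, sets its team, then applies the loadout through the mech's weapon handler after a fixed delay.
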(event Custom|EquipMech
  (params (mechWeaponHandler :type Mech%20Weapon%20Handler%20BP%20Object%20Reference))
  ;[1 1 1] Apply Loadout
  (Default|SetupLoadout mechWeaponHandler (Variables|Default|GetloadoutTemp))
  (Development|PrintString "Loadout"))

(event Custom|EventSpawnMech
  (params (Loadout :type Player%20Loadout%20Structure) (Team :type Team%20Enum :default "NewEnumerator0") (Player%20ID :type Integer))
  (Variables|Default|SetloadoutTemp Loadout)
  (bind _returnvalue (Game|SpawnActorfromClass "/Game/Blueprints/Mech_Pawn.Mech_Pawn_C" (Transformation|GetActorTransform) "AlwaysSpawn" 0 Player%20ID 0))
  (Variables|/Game/Blueprints/LivingActorComponent.LivingActorComponent_C|SetTeam (Variables|/Game/Blueprints/Mech_Pawn.Mech_Pawn_C|GetLivingActorComponent _returnvalue) Team)
  (Utilities|FlowControl|Delay 1e+01)
  (CallFunction|EquipMech (Variables|/Game/Blueprints/Mech_Pawn.Mech_Pawn_C|GetMechWeaponHandlerBP _returnvalue)))

(event EventBeginPlay
  (bind _player_id_to_spawn (Variables|Default|GetPlayer%20ID%20To%20Spawn))
  (Networking|SwitchHasAuthority
    (:Authority
      (bind _asmad_mechs_game_instance (Utilities|Casting|CastToMadMechsGameInstance (Game|GetGameInstance)))
      (if (!= (Utilities|Array|Get(acopy) (Variables|/Game/Blueprints/MainMenu/MadMechsGameInstance.MadMechsGameInstance_C|GetPlayerIDToSlot _asmad_mechs_game_instance) _player_id_to_spawn) -1)
        (CallFunction|EventSpawnMech (Utilities|Array|Get(acopy) (Variables|/Game/Blueprints/MainMenu/MadMechsGameInstance.MadMechsGameInstance_C|GetLoadouts _asmad_mechs_game_instance) _player_id_to_spawn) (Utilities|Array|Get(acopy) (Variables|/Game/Blueprints/MainMenu/MadMechsGameInstance.MadMechsGameInstance_C|GetTeams _asmad_mechs_game_instance) _player_id_to_spawn) (Utilities|Array|Get(acopy) (Variables|/Game/Blueprints/MainMenu/MadMechsGameInstance.MadMechsGameInstance_C|GetPlayerIDToSlot _asmad_mechs_game_instance) _player_id_to_spawn))))))

(event EventTick
  (params (DeltaSeconds :type Float%20%28single-precision%29)))

(fn ConstructionScript)