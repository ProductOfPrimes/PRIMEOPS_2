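; Mech controller that drives its controlled pawn with twin-stick style input, keeping walk direction separate from aim direction.
; Each tick, move input sets a target velocity that the current velocity approaches under an acceleration cap, then offsets the pawn with sweep.
; Velocity is stored as a per-frame displacement, from which speed and walk direction are derived, and a drag term is subtracted afterwards.
; Non-zero look input updates the normalized aim direction without rotating the pawn.
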(event EventTick
  (params (DeltaSeconds :type Float%20%28single-precision%29))
  (bind _returnvalue (Input|AxisValues|GetLookForward))
  (bind _returnvalue_2 (Input|AxisValues|GetLookRight))
  (bind _returnvalue_3 (Math|Vector|MakeVector _returnvalue _returnvalue_2 0.0))
  ;[1 1 1] Movement
  (Utilities|FlowControl|Sequence
    (:then_0
      (bind _output_get (Variables|Default|SetDesiredVelocity (* (Math|Vector|ClampVectorSize (Math|Vector|MakeVector (Input|AxisValues|GetMoveForward) (Input|AxisValues|GetMoveRight) 0.0) 0.0 1.0) (* DeltaSeconds (Variables|Default|GetSpeedMax)))))
      (bind _output_get_2 (Variables|Default|SetDesiredDeltaVelocity (- _output_get (Variables|Default|GetVelocity))))
      (bind _output_get_3 (Variables|Default|SetVelocity (+ (Math|Vector|VectorClampSizeMax _output_get_2 (* DeltaSeconds (Variables|Default|GetAccelerationMax))) (Variables|Default|GetVelocity))))
      (Variables|Default|SetSpeed (/ (Math|Vector|VectorLength _output_get_3) DeltaSeconds))
      (if (> (Math|Vector|VectorLength _output_get_3) 0.0)
        (Transformation|AddActorWorldOffset (Pawn|GetControlledPawn) _output_get_3 true)
        (Variables|Default|SetWalkDirection (Math|Vector|Normalize _output_get_3))))
    (:then_1
      (Variables|Default|SetVelocity (- (Variables|Default|GetVelocity) (* DeltaSeconds (Variables|Default|GetDrag)))))
    (:then_2
      (if (> (Math|Vector|VectorLength _returnvalue_3) 0.0)
        (Utilities|FlowControl|Sequence
          (:then_0
            (Variables|Default|SetAimDirection (Math|Vector|Normalize _returnvalue_3))))))))

(fn ConstructionScript)