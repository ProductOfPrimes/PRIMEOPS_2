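; Mech controller that drives walking and independent torso aim for the controlled pawn from move and look input on Tick.
; Input accelerates a clamped velocity, decayed by linear and exponential drag, whose speed moves the pawn along WalkDirection with a swept offset.
; A negative dot product between velocity and desired velocity triggers a gradual pivot toward the last input instead of following velocity.
; AimDirection rotates separately toward the look stick at TurnSpeed, while WalkRotation follows WalkDirection.
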(event EventTick
  (params (DeltaSeconds :type Float%20%28single-precision%29))
  (bind _returnvalue (Input|AxisValues|GetLookForward))
  (bind _returnvalue_2 (Input|AxisValues|GetLookRight))
  (bind _velocity (Variables|Movement|GetVelocity))
  (bind _returnvalue_3 (Math|Vector|MakeVector _returnvalue_2 _returnvalue 0.0))
  (Variables|Default|SetDT DeltaSeconds)
  ;[1 1 1] Movement
  (Utilities|FlowControl|Sequence
    (:then_0
      (bind _velocity_2 (Utilities|InputtoVelocity (Input|AxisValues|GetMoveForward) (Input|AxisValues|GetMoveRight) (Variables|Default|GetDT))
        (:%20%20
          (Variables|Movement|SetSpeed (/ (Math|Vector|VectorLength _velocity_2) (Variables|Default|GetDT)))
          (if (> (Math|Vector|VectorLength _velocity_2) 0.0)
            (bind _output_get (Variables|Movement|SetVelocityDotProduct (Math|Vector|DotProduct (Math|Vector|Normalize (Variables|Movement|GetVelocity)) (Math|Vector|Normalize (Variables|Movement|GetDesiredVelocity))))) ; This dot product will be negative when the vectors are opposite
            (if (< _output_get 0.0)
              (Variables|Movement|SetIsTurning true))))))
    (:then_1
      (if (Variables|Movement|GetIsTurning)
        (Utilities|TurnPlayer
          (:NewParam2
            (if (< (Variables|Movement|GetTurnAngle) 1e+01)
              (Variables|Movement|SetIsTurning false)
              (else
                (Variables|Movement|SetIsTurning true)))))
        (else
          (Variables|Movement|SetWalkDirection (Math|Vector|Normalize (select (> (Math|Vector|VectorLength _velocity) 0.0) _velocity (Variables|Movement|GetLastDirInput)))))))
    (:then_2
      (Utilities|MovePlayer))
    (:then_3
      (Utilities|DecaySpeed (Variables|Default|GetDT)))
    (:then_4
      ;[1 1 1] Torso Rotation
      (Utilities|FlowControl|Sequence
        (:then_0
          (if (> (Math|Vector|VectorLength _returnvalue_3) 0.0)
            (Variables|Aiming|SetAimTarget (Math|Vector|Normalize _returnvalue_3))))
        (:then_1
          (if (> (Math|Float|Absolute(Float) (Class|KismetMathLibrary|VectorCosineAngle2D (Variables|Aiming|GetAimTarget) (Variables|Aiming|GetAimDirection))) 0.1)
            (Variables|Aiming|SetAimDirection (Math|Vector|Normalize (Math|Vector|RotateVectorAroundAxis (Variables|Aiming|GetAimDirection) (* (Variables|Default|GetDT) (Variables|Aiming|GetTurn%20Speed) (Math|Float|Sign(Float) (Class|KismetMathLibrary|VectorCosineAngle2D (Variables|Aiming|GetAimTarget) (Variables|Aiming|GetAimDirection)))) "0.000000, 0,-1.000000")))))))
    (:then_5
      (Variables|Movement|SetWalkRotation (Math|Conversions|RotationFromXVector (Variables|Movement|GetWalkDirection))))))

(fn ConstructionScript)