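; Destructible building actor that takes damage, then crumbles and sinks away when killed.
; Any damage goes to LivingActorComponent and plays an explosion sound and dust burst.
; On death it unlocks the plane-constrained destructible mesh, shatters it with radius damage, then drops it without collision and destroys the actor.
; Momentum-based collision damage with a brief re-hit cooldown exists but is disconnected from the Hit event.
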(event EventBeginPlay
  (Class|PrimitiveComponent|SetConstraintMode (Variables|Components|GetBuilding) "XYPlane"))

(event Collision|EventHit
  (params (MyComp :type Primitive%20Component%20Object%20Reference) (Other :type Actor%20Object%20Reference) (OtherComp :type Primitive%20Component%20Object%20Reference) (bSelfMoved :type Boolean) (HitLocation :type Vector :default "0, 0, 0") (HitNormal :type Vector :default "0, 0, 0") (NormalImpulse :type Vector :default "0, 0, 0") (Hit :type Hit%20Result%20Structure%20%28by%20ref%29))
  ;[1 1 1] Collision Damage
)

(event Game|Damage|EventAnyDamage
  (params (Damage :type Float%20%28single-precision%29) (DamageType :type Damage%20Type%20Object%20Reference) (InstigatedBy :type Controller%20Object%20Reference) (DamageCauser :type Actor%20Object%20Reference))
  (bind _killingblow (Default|TakeDamage (Variables|Default|GetLivingActorComponent) Damage))
  (Audio|PlaySoundatLocation "/Game/Audio/Sound/Explode_New2_.Explode_New2_" (Transformation|GetActorLocation) "0, 0, 0" 1.0 1.0 0.0 0 0 0)
  (Effects|SpawnEmitteratLocation "/Game/VFX/PS_BuildingDust_Burst.PS_BuildingDust_Burst" (+ (Transformation|GetActorLocation) "0, 0,3000.000000") "0, 0, 0" "2.000000,2.000000,2.000000")
  (if _killingblow
    (Default|OnDeath (Variables|Default|GetLivingActorComponent))
    (|Deathresponse)))

(fn ConstructionScript
  (Class|DestructibleComponent|SetDestructibleMesh (Variables|Components|GetBuilding) (Variables|Default|GetMesh)))

(fn ResetPhysicsInvuln
  (Variables|Default|SetPhysicsHittable true))