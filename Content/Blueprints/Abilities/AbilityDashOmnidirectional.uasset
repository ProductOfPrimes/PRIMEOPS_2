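; Omnidirectional dash ability for a mech that plays audio and particles on activation.
; It adds a velocity impulse to the legs collision along the controller's move input at Speed, or re-adds the current velocity when input is zero, aligning the Niagara effect to that vector.
; It flags the movement component as dashing until deactivation.
; Each tick, the mesh spins at an exponentially eased rate driven by cooldown progress.
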(event Custom|OnDeactivate_1
  (Variables|/Game/Blueprints/Components/MechMovementComponent.MechMovementComponent_C|SetisDashing (Variables|/Game/Blueprints/Mech_Pawn.Mech_Pawn_C|GetMechMovementComponent (Variables|Default|GetMechOwner)) false))

(event EventBeginPlay
  (|CallParentFunction) ; This node is disabled and will not be called.\nDrag off pins to build functionality.
)

(event Collision|EventActorBeginOverlap
  (params (OtherActor :type Actor%20Object%20Reference))
  (|CallParentFunction OtherActor) ; This node is disabled and will not be called.\nDrag off pins to build functionality.
)

(event EventOnActivate
  (bind _mechowner (Variables|Default|GetMechOwner))
  (bind _mechmovementcomponent (Variables|/Game/Blueprints/Mech_Pawn.Mech_Pawn_C|GetMechMovementComponent _mechowner))
  (|CallParentFunction)
  (bind _asmech_script_controller (Utilities|Casting|CastToMechScriptController (Pawn|GetController _mechowner)))
  (Audio|Components|Audio|Play (Variables|Default|GetAudio) 0.0)
  (Niagara|ResetSystem (Variables|Default|GetNiagara))
  (Physics|SetPhysicsLinearVelocity (Variables|/Game/Blueprints/Mech_Pawn.Mech_Pawn_C|GetLegsCollision _mechowner) (Math|Vector|SelectVector (Variables|/Game/Blueprints/Components/MechMovementComponent.MechMovementComponent_C|GetLinearVelocity _mechmovementcomponent) (* (Math|Vector|Normalize (Variables|/Script/PRIMEOPS_2.MechScriptController|GetmoveInput _asmech_script_controller)) (Variables|Default|GetSpeed)) (Math|Vector|VectorIsNearlyZero (Variables|/Script/PRIMEOPS_2.MechScriptController|GetmoveInput _asmech_script_controller))) true "None")
  (Transformation|SetWorldRotation (Variables|Default|GetNiagara) (Math|Rotator|MakeRotfromX (Math|Vector|SelectVector (Variables|/Game/Blueprints/Components/MechMovementComponent.MechMovementComponent_C|GetLinearVelocity _mechmovementcomponent) (* (Math|Vector|Normalize (Variables|/Script/PRIMEOPS_2.MechScriptController|GetmoveInput _asmech_script_controller)) (Variables|Default|GetSpeed)) (Math|Vector|VectorIsNearlyZero (Variables|/Script/PRIMEOPS_2.MechScriptController|GetmoveInput _asmech_script_controller)))) false false)
  (Variables|/Game/Blueprints/Components/MechMovementComponent.MechMovementComponent_C|SetisDashing _mechmovementcomponent true))

(event EventOnCooldownFinish
  (|CallParentFunction))

(event EventTick
  (params (DeltaSeconds :type Float%20%28single-precision%29))
  (bind _percent (CallFunction|GetCooldownProgressPercentage))
  (bind _output_get (Variables|Default|SetspinRate (Math|Interpolation|Ease "ExpoIn" _percent 0.0 (Variables|Default|GetspinRateMax))))
  (Transformation|AddLocalRotation (Variables|Default|GetStaticMesh) (Math|Rotator|MakeRotator 0.0 0.0 (* _output_get DeltaSeconds)) false false))

(fn ConstructionScript
  (|CallParentFunction))