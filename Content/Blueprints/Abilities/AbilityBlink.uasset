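; Mech blink ability that, after a charge delay, hides the owner and dashes it along its move input.
; During the blink it ignores pawn, destructible and dynamic collision and disables leg collision.
; It then restores both and teleports the mech a further distance forward with a height offset; destination trace checks are disconnected.
; Tick spins the ability's mesh at a rate eased by cooldown progress.
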(event EventBeginPlay
  (|CallParentFunction) ; This node is disabled and will not be called.\nDrag off pins to build functionality.
)

(event Collision|EventActorBeginOverlap
  (params (OtherActor :type Actor%20Object%20Reference))
  (|CallParentFunction OtherActor) ; This node is disabled and will not be called.\nDrag off pins to build functionality.
)

(event EventOnActivate
  (bind _mechowner (Variables|Default|GetMechOwner))
  (bind _mechowner_2 (Variables|Default|GetMechOwner))
  (bind _mechowner_3 (Variables|Default|GetMechOwner))
  (bind _legs_01 (Variables|/Game/Blueprints/Mech_Pawn.Mech_Pawn_C|Getlegs_01 _mechowner_3))
  (bind _terraincollision (Variables|/Game/Blueprints/Mech_Pawn.Mech_Pawn_C|GetTerrainCollision _mechowner_3))
  (bind _mechmovementcomponent (Variables|/Game/Blueprints/Mech_Pawn.Mech_Pawn_C|GetMechMovementComponent _mechowner_2))
  (bind _moveinput (Variables|/Game/Blueprints/Mech_Pawn.Mech_Pawn_C|GetMoveInput _mechowner_2))
  (bind _returnvalue (Math|Vector|Normalize _moveinput))
  (|CallParentFunction)
  (Audio|Components|Audio|Play (Variables|Default|GetAudio) 0.0)
  (Utilities|FlowControl|Delay (Variables|Default|GetChargeTime))
  (Niagara|SpawnSystematLocation (Variables|Default|GetParticles) (Transformation|GetActorLocation _mechowner_2) (Math|Rotator|MakeRotfromX _returnvalue))
  (Variables|/Game/Blueprints/Components/MechMovementComponent.MechMovementComponent_C|SetisDashing _mechmovementcomponent true)
  (Physics|SetPhysicsLinearVelocity (Variables|/Game/Blueprints/Components/MechMovementComponent.MechMovementComponent_C|GetBodyPrimitive _mechmovementcomponent) (* _returnvalue (Variables|Default|GetSpeed)) true "None")
  (Rendering|SetVisibility (Variables|/Script/Engine.Actor|GetRootComponent _mechowner_3) false true)
  (Utilities|FlowControl|Sequence
    (:then_0
      (Collision|SetCollisionResponsetoChannel _terraincollision "ECC_Pawn" "ECR_Ignore")
      (Collision|SetCollisionResponsetoChannel _terraincollision "ECC_Destructible" "ECR_Ignore")
      (Collision|SetCollisionResponsetoChannel _terraincollision "ECC_WorldDynamic" "ECR_Ignore"))
    (:then_1
      (Collision|SetCollisionEnabled _legs_01 "NoCollision"))
    (:then_2
      (Utilities|FlowControl|Delay (Variables|Default|GetBlinkDuration))
      (Utilities|FlowControl|Sequence
        (:then_0
          (Collision|SetCollisionResponsetoChannel _terraincollision "ECC_Pawn" "ECR_Block")
          (Collision|SetCollisionResponsetoChannel _terraincollision "ECC_Destructible" "ECR_Block")
          (Collision|SetCollisionResponsetoChannel _terraincollision "ECC_WorldDynamic" "ECR_Block"))
        (:then_1
          (Collision|SetCollisionEnabled _legs_01 "QueryAndPhysics"))
        (:then_2
          (Rendering|SetVisibility (Variables|/Script/Engine.Actor|GetRootComponent (Variables|Default|GetMechOwner)) true true))
        (:then_3
          (CallFunction|TryTeleporttoDestination _mechowner (+ (+ (Transformation|GetActorLocation _mechowner) (* _returnvalue (Variables|Default|GetDistance))) "0.000000,0.000000,600.000000") 5.5e+02 (Collision|GetCollisionProfileName (Variables|/Game/Blueprints/Mech_Pawn.Mech_Pawn_C|GetTerrainCollision _mechowner)))
          (Variables|/Game/Blueprints/Components/MechMovementComponent.MechMovementComponent_C|SetisDashing (Variables|/Game/Blueprints/Mech_Pawn.Mech_Pawn_C|GetMechMovementComponent (Variables|Default|GetMechOwner)) false)
          (Niagara|ResetSystem (Variables|Default|GetNiagara)))))))

(event EventTick
  (params (DeltaSeconds :type Float%20%28single-precision%29))
  (|CallParentFunction DeltaSeconds)
  (bind _percent (CallFunction|GetCooldownProgressPercentage))
  (bind _output_get (Variables|Default|SetspinRate (Math|Interpolation|Ease "ExpoIn" _percent -1e+02 (Variables|Default|GetspinRateMax))))
  (Transformation|AddLocalRotation (Variables|Default|GetStaticMesh) (Math|Rotator|MakeRotator 0.0 0.0 (* _output_get DeltaSeconds)) false false))

(event EventOnCooldownFinish
  (|CallParentFunction))

(event EventOnDeactivate
  (|CallParentFunction))

(fn ConstructionScript
  (|CallParentFunction))

(fn TryTeleporttoDestination
  (params (Actor :type Actor%20Object%20Reference%20%28by%20ref%29) (Destination :type Vector) (CollisionRadius :type Float%20%28double-precision%29) (Collision%20Profile :type Name))
  (bind _output_get (LocalVariables|SetTargetLocation Destination))
  (bind _returnvalue (Transformation|Teleport (Variables|Default|GetMechOwner) (LocalVariables|GetTargetLocation) "0, 0, 0")) ; Teleport to target location
  (if _returnvalue
    _
    (else
      (Development|PrintString "Mech Too Phat!")))
  (return))