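; Base projectile actor for mech abilities that moves as a physics-driven mesh and damages what it strikes.
; Tick accumulates distance from the mesh's physics velocity and, past Range, spawns a self-destruct effect and destroys it.
; Physical hits and overlaps with non-instigator mech pawns (via a synthesized hit result) feed OnHitTarget.
; OnHitTarget plays impact FX and sound, applies point damage, then destroys the projectile.
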(event EventBeginPlay)

(event Collision|EventActorBeginOverlap
  (params (OtherActor :type Actor%20Object%20Reference))
  (bind _returnvalue (Transformation|GetActorLocation))
  (bind _returnvalue_2 (Transformation|GetActorForwardVector))
  (bind _asmech_pawn (Utilities|Casting|CastToMech_Pawn OtherActor))
  (if (!= _asmech_pawn (Variables|Actor|GetInstigator))
    (CallFunction|OnHitTarget (Collision|MakeHitResult false true 0.0 0.0 _returnvalue _returnvalue _returnvalue_2 (* _returnvalue_2 -1.0) 0 OtherActor))))

(event EventTick
  (params (DeltaSeconds :type Float%20%28single-precision%29))
  (bind _returnvalue (Physics|GetPhysicsLinearVelocity (Variables|Default|GetStaticMesh) "None"))
  (Utilities|FlowControl|Sequence
    (:then_0
      (if (> (+ (Variables|Gameplay|GetDistanceTravelled) (* DeltaSeconds (Math|Vector|VectorLength _returnvalue))) (Variables|Gameplay|GetRange)) ; If true, spawn some explosion particle or whatever and deleteparent()?
        (CallFunction|OnExpire)))
    (:then_1
      (Variables|Gameplay|SetDistanceTravelled (+ (Variables|Gameplay|GetDistanceTravelled) (* DeltaSeconds (Math|Vector|VectorLength _returnvalue))))
      (Variables|Default|SetvelocityLastFrame _returnvalue))))

(event Collision|EventHit
  (params (MyComp :type Primitive%20Component%20Object%20Reference) (Other :type Actor%20Object%20Reference) (OtherComp :type Primitive%20Component%20Object%20Reference) (bSelfMoved :type Boolean) (HitLocation :type Vector :default "0, 0, 0") (HitNormal :type Vector :default "0, 0, 0") (NormalImpulse :type Vector :default "0, 0, 0") (Hit :type Hit%20Result%20Structure%20%28by%20ref%29))
  (CallFunction|OnHitTarget Hit))

(fn ConstructionScript)

(fn OnExpire
  (Niagara|SpawnSystematLocation "/Game/VFX/NS_ProjectileSelfDestruct.NS_ProjectileSelfDestruct" (Transformation|GetWorldLocation (Variables|Default|GetStaticMesh)) "0, 0, 0" "1.000000,1.000000,1.000000" true true "AutoRelease")
  (Actor|DestroyActor))

(fn OnHitTarget
  (params (hit%20info :type Hit%20Result%20Structure%20%28by%20ref%29))
  (bind (_bblockinghit _binitialoverlap _time _distance _location _impactpoint _normal _impactnormal _physmat _hitactor) (Collision|BreakHitResult hit%20info))
  (Utilities|FlowControl|Sequence
    (:then_0
      (Niagara|SpawnSystematLocation (Variables|Default|GetHit%20FX) _impactpoint (Math|Rotator|MakeRotfromX (Math|Vector|GetForwardVector (Variables|Default|GetStaticMesh))) "1.000000,1.000000,1.000000" true true "AutoRelease")
      (CallFunction|PlaySoundatLocationwithVariance (Variables|Default|GetImpact%20Sound) _impactpoint 0.5 0.3))
    (:then_1
      (Game|Damage|ApplyPointDamage _hitactor (Variables|Gameplay|GetAttack) _normal hit%20info (Game|GetInstigatorController) (Variables|Gameplay|GetPlayerOwner) "/Script/Engine.DamageType"))
    (:then_2
      (Actor|DestroyActor))
    (:then_3
      (return))))

(fn GetDistanceTravelled
  (return (Variables|Gameplay|GetDistanceTravelled)))