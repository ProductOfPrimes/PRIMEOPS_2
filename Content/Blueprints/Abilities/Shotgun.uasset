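; Shotgun ability Blueprint that builds on a parent ability class, leaving firing and cooldown-finish behavior to that parent.
; Each tick it calls SetHeatMaterialParameter to update a heat material parameter.
; On activation it runs the parent logic, then waits until shortly before the cooldown ends to play ShotgunReload.
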(event EventBeginPlay
  (|CallParentFunction) ; This node is disabled and will not be called.\nDrag off pins to build functionality.
)

(event Collision|EventActorBeginOverlap
  (params (OtherActor :type Actor%20Object%20Reference))
  (|CallParentFunction OtherActor) ; This node is disabled and will not be called.\nDrag off pins to build functionality.
)

(event EventTick
  (params (DeltaSeconds :type Float%20%28single-precision%29))
  (|CallParentFunction DeltaSeconds)
  (CallFunction|SetHeatMaterialParameter))

(event EventOnActivate
  (|CallParentFunction)
  (Utilities|FlowControl|Delay (- (Variables|Default|GetCooldown) 0.3))
  (Audio|Components|Audio|Play (Variables|Default|GetShotgun_Reload) 0.0))

(event EventOnCooldownFinish
  (|CallParentFunction))

(fn ConstructionScript
  (|CallParentFunction))

(fn Fire
  (|CallParentFunction))