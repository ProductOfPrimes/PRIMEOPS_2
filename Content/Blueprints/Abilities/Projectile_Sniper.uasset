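; Sniper projectile Blueprint that adds a Niagara trail to behavior inherited from its parent class.
; BeginPlay spawns the trail attached to the static mesh, with auto-destroy and auto-release pooling.
; On Destroyed, the trail detaches keeping its world transform, so it is left in place rather than following the projectile.
; Overlap and Tick are disabled, and some leftover debug nodes are unconnected.
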(event EventBeginPlay
  (|CallParentFunction)
  (bind _returnvalue (Niagara|SpawnSystemAttached (Variables|Default|GetNiagara%20Trail) (Variables|Default|GetStaticMesh) "None" "0, 0, 0" "0, 0, 0" "KeepRelativeOffset" true true "AutoRelease")))

(event Collision|EventActorBeginOverlap
  (params (OtherActor :type Actor%20Object%20Reference))
  (|CallParentFunction OtherActor) ; This node is disabled and will not be called.\nDrag off pins to build functionality.
)

(event EventTick
  (params (DeltaSeconds :type Float%20%28single-precision%29))
  (|CallParentFunction DeltaSeconds) ; This node is disabled and will not be called.\nDrag off pins to build functionality.
)

(event EventDestroyed
  (Transformation|DetachFromComponent (stale EventBeginPlay _returnvalue) "KeepWorld" "KeepWorld" "KeepWorld" true))

(fn ConstructionScript
  (|CallParentFunction))