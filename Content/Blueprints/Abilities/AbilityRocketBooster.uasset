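; Mech rocket booster ability that pushes the body along its center-of-thrust forward vector while active.
; Activation starts audio and two Niagara effects and flags the movement component as dashing; deactivation undoes these.
; Each tick while thrusting, it adds radiator heat, shuts off on overheat, otherwise applies acceleration force.
; It also feeds the 2D-clamped physics velocity into the movement component's desired velocity offset.
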(event EventBeginPlay
  (|CallParentFunction) ; This node is disabled and will not be called.\nDrag off pins to build functionality.
)

(event Collision|EventActorBeginOverlap
  (params (OtherActor :type Actor%20Object%20Reference))
  (|CallParentFunction OtherActor) ; This node is disabled and will not be called.\nDrag off pins to build functionality.
)

(event EventTick
  (params (DeltaSeconds :type Float%20%28single-precision%29))
  (bind _mechowner (Variables|Default|GetMechOwner))
  (bind _mechmovementcomponent (Variables|/Game/Blueprints/Mech_Pawn.Mech_Pawn_C|GetMechMovementComponent _mechowner))
  (bind _bodyprimitive (Variables|/Game/Blueprints/Components/MechMovementComponent.MechMovementComponent_C|GetBodyPrimitive _mechmovementcomponent))
  (CallFunction|SetHeatMaterialParameter)
  (if (Variables|Default|Getthrusting)
    (Default|AddHeat (Variables|/Game/Blueprints/Mech_Pawn.Mech_Pawn_C|GetMechRadiator (Variables|Default|GetMechOwner)) (* (Variables|Default|GetHeatGeneration) DeltaSeconds))
    (if (Variables|/Game/Blueprints/MechRadiator.MechRadiator_C|GetOverheated (Variables|/Game/Blueprints/Mech_Pawn.Mech_Pawn_C|GetMechRadiator _mechowner))
      (CallFunction|DeactivateAbility)
      (else
        (Physics|AddForce _bodyprimitive (* (Math|Vector|GetForwardVector (Variables|Default|GetCenter%20of%20Thrust)) (Variables|Default|GetThrust)) "None" true)
        (bind _returnvalue (Physics|GetPhysicsLinearVelocity _bodyprimitive "None"))
        (Variables|/Game/Blueprints/Components/MechMovementComponent.MechMovementComponent_C|SetDesiredVelocityOffset _mechmovementcomponent (Class|KismetMathLibrary|VectorClampSizeMax2D _returnvalue (Variables|Default|GetDesiredSpeedOverrideMagnitudeCap)))))))

(event EventOnActivate)

(event EventOnDeactivate
  (bind _mechowner (Variables|Default|GetMechOwner))
  (bind _mechmovementcomponent (Variables|/Game/Blueprints/Mech_Pawn.Mech_Pawn_C|GetMechMovementComponent _mechowner))
  (|CallParentFunction)
  (Components|Activation|Deactivate (Variables|Default|GetNiagara))
  (Audio|Components|Audio|Stop (Variables|Default|GetAudio))
  (Variables|/Game/Blueprints/Components/MechMovementComponent.MechMovementComponent_C|SetisDashing _mechmovementcomponent false)
  (Variables|Default|Setthrusting false)
  (Variables|/Game/Blueprints/Components/MechMovementComponent.MechMovementComponent_C|SetDesiredVelocityOffset _mechmovementcomponent "0, 0, 0"))

(fn ConstructionScript
  (|CallParentFunction))

(fn ActivateAbility
  (if (not (Variables|Default|Getthrusting))
    (Audio|Components|Audio|Play (Variables|Default|GetAudio) 0.0)
    (Components|Activation|Activate (Variables|Default|GetNiagara) false)
    (Variables|/Game/Blueprints/Components/MechMovementComponent.MechMovementComponent_C|SetisDashing (Variables|/Game/Blueprints/Mech_Pawn.Mech_Pawn_C|GetMechMovementComponent (Variables|Default|GetMechOwner)) true)
    (Variables|Default|Setthrusting true)))