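; Base actor Blueprint for mech abilities, providing a shared cooldown and a stored MechOwner reference.
; Tick counts CooldownTimer down, sets OnCooldown while it is non-negative, and fires a finish event once when it drops below zero.
; Activate, OnEquip, OnUnequip and OnCooldownFinish are empty hooks, and nothing here starts the cooldown.
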(event Custom|Event%20OnUnequip)

(event Custom|Event%20OnEquip)

(event Custom|Event%20OnCooldownFinish)

(event EventBeginPlay)

(event Collision|EventActorBeginOverlap
  (params (OtherActor :type Actor%20Object%20Reference)))

(event EventTick
  (params (DeltaSeconds :type Float%20%28single-precision%29))
  (bind _output_get (Variables|AbilityProperties|SetCooldownTimer (- (Variables|AbilityProperties|GetCooldownTimer) DeltaSeconds)))
  (if (< _output_get 0.0)
    ;[1 1 1] Invoke OnCooldownFinish once CooldownTimer hits 0.0
    (if (Variables|AbilityProperties|GetOnCooldown)
      (Variables|AbilityProperties|SetCooldownTimer 0.0)
      (Variables|AbilityProperties|SetOnCooldown false)
      (CallFunction|EventonCooldownFinish))
    (else
      (Variables|AbilityProperties|SetOnCooldown true))))

(fn ConstructionScript)

(fn Activate)

(fn SetMechOwner
  (params (owner :type Mech%20Controller%20Object%20Reference))
  (Variables|Components|SetMechOwner owner))