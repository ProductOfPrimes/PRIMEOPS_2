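; Projectile variant that deals area-of-effect damage to mechs and buildings on impact.
; OnHitTarget spawns hit FX and a pitch-varied sound at the SplashRadius sphere, applies splash damage, then destroys the projectile.
; Mechs and buildings overlapping the sphere take Attack damage, each group toggled by a flag and credited to PlayerOwner's instigator controller.
; Mechs also receive a linear-falloff radial knockback on their TerrainCollision.
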(event EventBeginPlay
  (|CallParentFunction) ; This node is disabled and will not be called.\nDrag off pins to build functionality.
)

(event Collision|EventActorBeginOverlap
  (params (OtherActor :type Actor%20Object%20Reference))
  (|CallParentFunction OtherActor) ; This node is disabled and will not be called.\nDrag off pins to build functionality.
)

(event EventTick
  (params (DeltaSeconds :type Float%20%28single-precision%29))
  (|CallParentFunction DeltaSeconds) ; This node is disabled and will not be called.\nDrag off pins to build functionality.
)

(fn ConstructionScript
  (|CallParentFunction))

(fn OnHitTarget
  (params (hit%20info :type Hit%20Result%20Structure%20%28by%20ref%29))
  (bind _splashradius (Variables|Default|GetSplashRadius))
  (bind _returnvalue (Transformation|GetWorldLocation _splashradius))
  (Utilities|FlowControl|Sequence
    (:then_0
      (Niagara|SpawnSystematLocation (Variables|Default|GetHit%20FX) _returnvalue (Math|Rotator|MakeRotfromX (Math|Vector|GetForwardVector (Variables|Default|GetStaticMesh))) "1.000000,1.000000,1.000000" true true "AutoRelease")
      (CallFunction|PlaySoundatLocationwithVariance (Variables|Default|GetImpact%20Sound) _returnvalue 1.0 0.15))
    (:then_1
      (CallFunction|ApplySplashDamage))
    (:then_2
      (Actor|DestroyActor)
      (return))))

(fn ApplySplashDamage
  (bind _splashradius (Variables|Default|GetSplashRadius))
  (bind _splashradius_2 (Variables|Default|GetSplashRadius))
  (if (Variables|Default|GetDealDamageToMechs)
    (for _array_element (Collision|GetOverlappingActors _splashradius "/Game/Blueprints/Mech_Pawn.Mech_Pawn_C" :!class /Script/Engine.PrimitiveComponent)
      (Game|Damage|ApplyDamage _array_element (Variables|Default|GetAttack) (Game|GetInstigatorController (Variables|Default|GetPlayerOwner)) self "/Script/Engine.DamageType")
      (bind _asmech_pawn (Utilities|Casting|CastToMech_Pawn _array_element))
      (Physics|AddRadialForce (Variables|/Game/Blueprints/Mech_Pawn.Mech_Pawn_C|GetTerrainCollision _asmech_pawn) (Transformation|GetWorldLocation _splashradius_2) (Components|Sphere|GetScaledSphereRadius _splashradius_2) (Variables|Default|GetKnockback) "RIF_Linear" true)))
  (if (Variables|Default|GetDealDamageToBuildings)
    (for _array_element_2 (Collision|GetOverlappingActors _splashradius "/Game/Blueprints/BP_Building.BP_Building_C" :!class /Script/Engine.PrimitiveComponent)
      (Game|Damage|ApplyDamage _array_element_2 (Variables|Default|GetAttack) (Game|GetInstigatorController (Variables|Default|GetPlayerOwner)) self "/Script/Engine.DamageType"))))