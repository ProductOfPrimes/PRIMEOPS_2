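; Grenade projectile Blueprint that launches its physics-driven StaticMesh on BeginPlay.
; The launch sets linear velocity along the mesh's right vector, scaled by Speed.
; Each Tick calls the parent and re-orients the mesh with world up, blending actor forward slightly toward velocity, and prints that rotation to screen as debug.
; It adds no impact or detonation logic of its own.
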(event EventBeginPlay
  (bind _staticmesh (Variables|Default|GetStaticMesh))
  (|CallParentFunction)
  (bind _result (Math|Float|NegateFloat (Variables|Default|GetSpeed))
    (:%20%20
      (Physics|SetPhysicsLinearVelocity _staticmesh (* (Math|Vector|GetRightVector _staticmesh) _result) false "None"))))

(event Collision|EventActorBeginOverlap
  (params (OtherActor :type Actor%20Object%20Reference))
  (|CallParentFunction OtherActor) ; This node is disabled and will not be called.\nDrag off pins to build functionality.
)

(event EventTick
  (params (DeltaSeconds :type Float%20%28single-precision%29))
  (bind _returnvalue (Transformation|GetVelocity))
  (bind _returnvalue_2 (Transformation|GetActorForwardVector))
  (bind _returnvalue_3 (Math|Vector|VectorUp))
  (bind _returnvalue_4 (Math|Vector|Lerp(Vector) _returnvalue_2 _returnvalue 0.01))
  (bind _returnvalue_5 (Math|Rotator|MakeRotfromXZ _returnvalue_4 _returnvalue_3))
  (Transformation|SetWorldRotation (Variables|Default|GetStaticMesh) _returnvalue_5 false false)
  (|CallParentFunction DeltaSeconds)
  (Development|PrintString (Utilities|String|ToString(Rotator) _returnvalue_5)))

(fn ConstructionScript
  (|CallParentFunction))