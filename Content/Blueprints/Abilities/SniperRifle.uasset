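; Sniper rifle weapon ability for a mech, which fires a straight projectile.
; Fire spawns a Projectile_Straight at the transform of the pawn controlled by MechOwner and prints a debug message.
; GetType identifies the weapon with an enum value, and the construction script calls its parent before printing a debug label.
; The event graph holds only disabled placeholder events.
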(event EventBeginPlay
  (|CallParentFunction) ; This node is disabled and will not be called.\nDrag off pins to build functionality.
)

(event Collision|EventActorBeginOverlap
  (params (OtherActor :type Actor%20Object%20Reference))
  (|CallParentFunction OtherActor) ; This node is disabled and will not be called.\nDrag off pins to build functionality.
)

(event EventTick
  (params (DeltaSeconds :type Float%20%28single-precision%29))
  (|CallParentFunction DeltaSeconds) ; This node is disabled and will not be called.\nDrag off pins to build functionality.
)

(fn ConstructionScript
  (Utilities|FlowControl|Sequence
    (:then_0
      (|CallParentFunction))
    (:then_1
      (Development|PrintString "Sniper"))))

(fn GetType
  (return "NewEnumerator1"))

(fn Fire
  (Game|SpawnActorfromClass "/Game/Blueprints/Abilities/Projectile_Straight.Projectile_Straight_C" (Transformation|GetActorTransform (Pawn|GetControlledPawn (Variables|Default|GetMechOwner))) "Undefined" 0 0)
  (Development|PrintString "Sniper Fired"))