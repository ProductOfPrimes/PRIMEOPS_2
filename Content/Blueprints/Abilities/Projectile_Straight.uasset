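; Straight-flying projectile ability that knocks mechs back and can ricochet off them on glancing impacts.
; Hit and overlap events apply knockback along the projectile's forward vector, with overlaps ignoring the owning player and building a synthetic hit result.
; RichochetCheck derives a normal from the mech's center, and shallow impacts within the deflect limit reflect velocity and rotation with sparks and sound.
; Other impacts call OnHitTarget.
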(event EventBeginPlay)

(event Collision|EventActorBeginOverlap
  (params (OtherActor :type Actor%20Object%20Reference))
  (bind _returnvalue (Transformation|GetActorLocation))
  (bind _returnvalue_2 (Transformation|GetActorForwardVector))
  (bind _returnvalue_3 (* _returnvalue_2 -1.0))
  (bind _returnvalue_4 (Collision|MakeHitResult false true 0.0 0.0 _returnvalue _returnvalue _returnvalue_2 _returnvalue_3 0 OtherActor))
  (bind _asmech_pawn (Utilities|Casting|CastToMech_Pawn OtherActor)
    (:then
      (if (!= _asmech_pawn (Variables|Default|GetPlayerOwner))
        (CallFunction|ApplyKnockback _asmech_pawn)
        (bind _did_ricochet_ (CallFunction|RichochetCheck _returnvalue_4))
        (if (not _did_ricochet_)
          (CallFunction|OnHitTarget _returnvalue_4 :!label _label))))
    (:CastFailed
      (goto _label))))

(event EventTick
  (params (DeltaSeconds :type Float%20%28single-precision%29))
  (|CallParentFunction DeltaSeconds))

(event Collision|EventHit
  (params (MyComp :type Primitive%20Component%20Object%20Reference) (Other :type Actor%20Object%20Reference) (OtherComp :type Primitive%20Component%20Object%20Reference) (bSelfMoved :type Boolean) (HitLocation :type Vector :default "0, 0, 0") (HitNormal :type Vector :default "0, 0, 0") (NormalImpulse :type Vector :default "0, 0, 0") (Hit :type Hit%20Result%20Structure%20%28by%20ref%29))
  (bind _asmech_pawn (Utilities|Casting|CastToMech_Pawn Other)
    (:then
      (CallFunction|ApplyKnockback _asmech_pawn)
      (bind _did_ricochet_ (CallFunction|RichochetCheck Hit))
      (if (not _did_ricochet_)
        (CallFunction|OnHitTarget Hit :!label _label)))
    (:CastFailed
      (goto _label))))

(fn ConstructionScript
  (|CallParentFunction))

(fn RichochetCheck
  (params (hit%20info :type Hit%20Result%20Structure))
  (bind (_bblockinghit _binitialoverlap _time _distance _location _impactpoint _normal _impactnormal _physmat _hitactor) (Collision|BreakHitResult hit%20info))
  (bind _staticmesh (Variables|Default|GetStaticMesh))
  (bind _returnvalue (Transformation|GetActorLocation _hitactor))
  (bind _returnvalue_2 (Math|Vector|GetForwardVector _staticmesh))
  (bind _returnvalue_3 (- _impactpoint _returnvalue))
  (if (< (Variables|Default|GetdeflectCount) (Variables|Default|GetdeflectMax)) ; Any Ricochets left? If not then die
    (bind _output_get (LocalVariables|SetRicochet%20Normal (/ _returnvalue_3 (Math|Vector|VectorLengthXY _returnvalue_3))))
    (if (< (* (Math|Vector|DotProduct _output_get (Math|Vector|ProjectVectorontoPlane _returnvalue_2 "0, 0,1.000000")) -1.0) (Variables|Default|GetRicochetDot)) ; final ricochet check
      ;[1 1 1] Ricochet response
      (Utilities|FlowControl|Sequence
        (:then_0
          (Math|Integer|IncrementInt (Variables|Default|GetdeflectCount)))
        (:then_1
          (Physics|SetPhysicsLinearVelocity (Variables|Default|GetStaticMesh) (* (Math|Vector|GetReflectionVector _returnvalue_2 _output_get) (Variables|Default|GetSpeed)) false "None")
          (Transformation|SetWorldRotation (Variables|Default|GetStaticMesh) (Math|Rotator|MakeRotfromXZ (Math|Vector|GetReflectionVector _returnvalue_2 _output_get) (Math|Vector|VectorUp)) false true))
        (:then_2
          (Niagara|SpawnSystematLocation "/Game/VFX/Impacts/NS_RicochetSparks.NS_RicochetSparks" _impactpoint (Math|Rotator|MakeRotfromX _output_get) "1.000000,1.000000,1.000000" true true "AutoRelease")
          (CallFunction|PlayRandomSoundatLocationwithVariance (Variables|Default|GetRicochetSounds) _impactpoint 1.0 0.3))
        (:then_3
          (return true)))
      (else
        (return false)))
    (else
      (CallFunction|OnHitTarget hit%20info))))

(fn ApplyKnockback
  (params (Mech :type Mech%20Pawn%20Object%20Reference))
  ;[1 1 1] Calculate Knockback
  (Default|AddKnockback (Variables|/Game/Blueprints/Mech_Pawn.Mech_Pawn_C|GetMechMovementComponent Mech) (* (Math|Vector|GetForwardVector (Variables|Default|GetStaticMesh)) (Variables|Default|GetKnockback))))