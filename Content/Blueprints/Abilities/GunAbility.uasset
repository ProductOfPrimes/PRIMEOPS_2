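; Mech gun ability that fires bursts of physics-driven projectiles, adding heat to the mech's radiator and knocking it back on activation.
; ActivateAbility queues the burst, then Tick calls Fire on a shot timer, dims materials after the last shot and eases the mesh's recoil through cooldown.
; Fire randomizes direction within a spread cone, optionally flattened to a plane; spread grows per shot and recovers off cooldown.
; Vertical targeting is unfinished and disconnected.
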(event EventTick
  (params (DeltaSeconds :type Float%20%28single-precision%29))
  (bind _cooldown (Variables|Default|GetCooldown))
  (|CallParentFunction DeltaSeconds)
  (if (Variables|Default|GetOnCooldown)
    (if (> (Variables|Dynamic|GetBulletsToFire) 0)
      (bind _output_get (Variables|Dynamic|SetBurstShotCooldownTimer (- (Variables|Dynamic|GetBurstShotCooldownTimer) DeltaSeconds)))
      (while (< (Variables|Dynamic|GetBurstShotCooldownTimer) 0.0)
        (Variables|Dynamic|SetBurstShotCooldownTimer (+ _output_get (Variables|WeaponProperties|GetBurstShotCooldown)))
        (Math|Integer|DecrementInt (Variables|Dynamic|GetBulletsToFire)
          (:%20%20
            (CallFunction|Fire)
            (if (== (Variables|Dynamic|GetBulletsToFire) 0)
              (Variables|Default|SetCooldownTimer (Variables|Default|GetCooldown))
              (Variables|Dynamic|SetBurstShotCooldownTimer 0.0)
              (for _array_element (Variables|Default|GetDynamic%20Materials)
                (Rendering|Material|SetVectorParameterValue _array_element "ParamColorMultiply" "(R=0.239583,G=0.239583,B=0.239583,A=1.000000)" :!class /Script/Engine.MaterialInstanceDynamic))))))
      (CallFunction|PlaySoundatLocationwithVariance (Variables|Cosmeticproperties|GetFiring%20Sound) (Transformation|GetActorLocation) 1.0 (Variables|Cosmeticproperties|GetSound%20Pitch%20Variance))
      (else
        (Transformation|SetRelativeLocation (Variables|Default|GetStaticMesh) (Math|Interpolation|Ease :Function "ExpoIn" :Alpha (Math|Float|Clamp(Float) (/ (- _cooldown (Variables|Default|GetCooldownTimer)) _cooldown)) :A (* (* (Math|Vector|GetForwardVector (Variables|/Script/Engine.SceneComponent|GetRelativeRotation (Variables|Default|GetBullet%20Spawn))) (Variables|Default|GetRecoilMovement)) "1.000000,1.000000, 0")) false false)))
    (else
      (Utilities|RecoverSpread))))

(fn ConstructionScript
  (|CallParentFunction))

(fn Fire
  (bind _mechowner (Variables|Default|GetMechOwner))
  (bind _bullet_spawn (Variables|Default|GetBullet%20Spawn))
  (bind _spread (Variables|Dynamic|GetSpread))
  (bind _returnvalue (Math|Vector|GetForwardVector _bullet_spawn))
  (bind _returnvalue_2 (Math|Random|RandomUnitVectorinConeinDegrees _returnvalue _spread))
  (bind _returnvalue_3 (Game|SpawnActorfromClass (Variables|WeaponProperties|GetProjectile%20Class) (Math|Transform|MakeTransform (Transformation|GetWorldLocation _bullet_spawn) (Math|Rotator|MakeRotfromXZ (select (Variables|WeaponProperties|GetSpawnOnXYPlane) (Math|Vector|ProjectVectorontoPlane _returnvalue_2 (Math|Vector|GetUpVector _bullet_spawn)) _returnvalue_2) (Math|Vector|GetUpVector (Variables|Default|GetBullet%20Spawn))) (Transformation|GetWorldScale _bullet_spawn)) "AlwaysSpawn" "SelectDefaultAtRuntime" _mechowner (Variables|WeaponProperties|GetSpeed) (Variables|WeaponProperties|GetAttack) (Variables|WeaponProperties|GetRange) (Variables|WeaponProperties|GetKnockback) (Variables|/Game/Blueprints/Mech_Pawn.Mech_Pawn_C|GetTeam _mechowner) _mechowner _mechowner))
  (Utilities|IsValid _returnvalue_3
    (:Is%20Valid
      (bind _output_get (LocalVariables|SetSpawned%20Projectile _returnvalue_3))
      (Physics|SetPhysicsLinearVelocity (Variables|/Game/Blueprints/Abilities/Projectile_Base.Projectile_Base_C|GetStaticMesh (LocalVariables|GetSpawned%20Projectile)) (* (Transformation|GetActorForwardVector (LocalVariables|GetSpawned%20Projectile)) (Variables|WeaponProperties|GetSpeed)) false "None")
      (Niagara|ResetSystem (Variables|Default|GetMuzzleFlash))
      (Utilities|AddSpread)
      (return (LocalVariables|GetSpawned%20Projectile)))))

(fn ActivateAbility
  (if (== (Variables|Dynamic|GetBulletsToFire) 0)
    (Variables|Dynamic|SetBulletsToFire (Variables|WeaponProperties|GetBurstCount))
    (Variables|Default|SetCooldownTimer (Variables|Default|GetCooldown))
    (Default|AddHeat (Variables|/Game/Blueprints/Mech_Pawn.Mech_Pawn_C|GetMechRadiator (Variables|Default|GetMechOwner)) (Variables|Default|GetHeatGeneration))
    (CallFunction|OnActivate)
    (CallFunction|TriggerRecoil)))

(fn TriggerRecoil
  (Default|AddKnockback (Variables|/Game/Blueprints/Mech_Pawn.Mech_Pawn_C|GetMechMovementComponent (Variables|Default|GetMechOwner)) (* (Math|Vector|GetForwardVector (Variables|Default|GetBullet%20Spawn)) (* (Variables|WeaponProperties|GetRecoil) -1.0))))

(fn VerticalTargetingUpdate
  (bind _bullet_spawn (Variables|Default|GetBullet%20Spawn))
  (bind _returnvalue (Transformation|GetWorldLocation _bullet_spawn))
  (bind _returnvalue_2 (- _returnvalue "0, 0,300.000000"))
  (bind (_outhit _returnvalue_3) (Class|KismetSystemLibrary|SphereTraceSinglebyProfile _returnvalue_2 (+ _returnvalue_2 (* (Math|Vector|GetRightVector (Variables|Default|GetRoot)) (* (Variables|WeaponProperties|GetRange) -1.0))) 1e+02 (Collision|GetCollisionProfileName (Variables|Default|GetStaticMesh)) false 0 "ForOneFrame" true "(R=1.000000,G=0.000000,B=0.000000,A=1.000000)" "(R=0.000000,G=1.000000,B=0.000000,A=1.000000)" 1.0))
  (if _returnvalue_3
    _))