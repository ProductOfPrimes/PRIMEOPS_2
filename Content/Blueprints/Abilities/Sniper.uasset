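; Sniper weapon ability for a mech, extending a parent ability that handles firing and cooldown.
; Each tick it runs a long visibility trace from the bullet spawn, drawn only as a one-frame debug line, and updates a heat material parameter.
; Activation waits a fraction of the cooldown, then ejects a physics shell casing with randomized force and torque.
; Projectile path prediction and mutual collision-ignore nodes are present but never run.
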(event EventBeginPlay
  (|CallParentFunction) ; This node is disabled and will not be called.\nDrag off pins to build functionality.
)

(event Collision|EventActorBeginOverlap
  (params (OtherActor :type Actor%20Object%20Reference))
  (|CallParentFunction OtherActor) ; This node is disabled and will not be called.\nDrag off pins to build functionality.
)

(event EventTick
  (params (DeltaSeconds :type Float%20%28single-precision%29))
  (bind _bullet_spawn (Variables|Default|GetBullet%20Spawn))
  (bind _returnvalue (Transformation|GetWorldLocation _bullet_spawn))
  (|CallParentFunction DeltaSeconds)
  (Collision|LineTraceByChannel _returnvalue (+ _returnvalue (* (Math|Vector|GetForwardVector _bullet_spawn) 3e+04)) "TraceTypeQuery1" false 0 "ForOneFrame" true "(R=1.000000,G=0.000000,B=0.000000,A=1.000000)" "(R=0.520833,G=0.000000,B=0.005181,A=1.000000)" 1.0)
  (CallFunction|SetHeatMaterialParameter))

(event EventOnActivate
  (|CallParentFunction)
  (Utilities|FlowControl|Delay (* (Variables|Default|GetCooldown) 0.4))
  (CallFunction|SpawnShellCasing))

(event EventOnCooldownFinish
  (|CallParentFunction))

(fn ConstructionScript
  (|CallParentFunction))

(fn Fire
  (|CallParentFunction))

(fn SpawnShellCasing
  (bind _casingspawn (Variables|Default|GetCasingSpawn))
  (bind _returnvalue (Math|Vector|GetRightVector _casingspawn))
  (bind _returnvalue_2 (Game|SpawnActorfromClass "/Game/Blueprints/Abilities/Models/BP_shellcasing.BP_shellcasing_C" (Transformation|GetWorldTransform _casingspawn) "AlwaysSpawn" "MultiplyWithRoot" 0 0))
  (Physics|AddForce (Variables|/Script/Engine.StaticMeshActor|GetStaticMeshComponent _returnvalue_2) (* (Math|Random|RandomUnitVectorinConeinDegrees _returnvalue 5.0) 8e+04) "None" true)
  (Class|PrimitiveComponent|AddTorqueinDegrees (Variables|/Script/Engine.StaticMeshActor|GetStaticMeshComponent _returnvalue_2) (* (Math|Random|RandomUnitVectorinConeinDegrees _returnvalue 1.8e+02) 5e+04) "None" true))