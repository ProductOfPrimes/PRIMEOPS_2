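; Rocket boost ability for a mech, pushing it along the center-of-thrust forward vector and flagging it as dashing.
; On activation it applies a single mass-independent AddForce to the movement component's body, with no per-tick force in this graph.
; It also starts audio, a point light and a Niagara effect rotated to the thrust direction.
; Deactivation stops the audio and light and clears the dashing and thrusting flags.
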(event EventBeginPlay
  (|CallParentFunction) ; This node is disabled and will not be called.\nDrag off pins to build functionality.
)

(event Collision|EventActorBeginOverlap
  (params (OtherActor :type Actor%20Object%20Reference))
  (|CallParentFunction OtherActor) ; This node is disabled and will not be called.\nDrag off pins to build functionality.
)

(event EventOnActivate
  (bind _niagara (Variables|Default|GetNiagara))
  (bind _center_of_thrust (Variables|Default|GetCenter%20of%20Thrust))
  (bind _thrust (Variables|Default|GetThrust))
  (bind _returnvalue (Math|Vector|GetForwardVector _center_of_thrust))
  (bind _returnvalue_2 (* _returnvalue _thrust))
  (|CallParentFunction)
  (Audio|Components|Audio|Play (Variables|Default|GetAudio) 0.0)
  (Physics|AddForce (Variables|/Game/Blueprints/Components/MechMovementComponent.MechMovementComponent_C|GetBodyPrimitive (Variables|/Game/Blueprints/Mech_Pawn.Mech_Pawn_C|GetMechMovementComponent (Variables|Default|GetMechOwner))) _returnvalue_2 "None" true)
  (Transformation|SetWorldRotation _niagara (Math|Rotator|MakeRotfromX _returnvalue_2) false false)
  (Components|Activation|Activate (Variables|Default|GetPointLight) false)
  (Niagara|ResetSystem _niagara)
  (Variables|/Game/Blueprints/Components/MechMovementComponent.MechMovementComponent_C|SetisDashing (Variables|/Game/Blueprints/Mech_Pawn.Mech_Pawn_C|GetMechMovementComponent (Variables|Default|GetMechOwner)) true)
  (Variables|Default|Setthrusting true))

(event EventOnDeactivate
  (|CallParentFunction)
  (Components|Activation|Deactivate (Variables|Default|GetPointLight))
  (Audio|Components|Audio|Stop (Variables|Default|GetAudio))
  (Variables|/Game/Blueprints/Components/MechMovementComponent.MechMovementComponent_C|SetisDashing (Variables|/Game/Blueprints/Mech_Pawn.Mech_Pawn_C|GetMechMovementComponent (Variables|Default|GetMechOwner)) false)
  (Variables|Default|Setthrusting false))

(fn ConstructionScript
  (|CallParentFunction))