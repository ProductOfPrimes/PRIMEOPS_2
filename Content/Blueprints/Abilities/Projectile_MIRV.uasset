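; MIRV projectile ability that splits into submunitions as it descends.
; Tick points the spinning mesh along its physics velocity and triggers the split once it falls below an altitude and vertical velocity threshold.
; The split spawns submunitions ejected randomly in the plane perpendicular to the mesh's forward axis, each inheriting the parent's velocity plus a random share of ejection speed, then plays a sound and expires the parent.
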(event EventTick
  (params (DeltaSeconds :type Float%20%28single-precision%29))
  (bind _staticmesh (Variables|Default|GetStaticMesh))
  (bind _returnvalue (Physics|GetPhysicsLinearVelocity _staticmesh "None"))
  (Transformation|SetWorldRotation _staticmesh (Math|Rotator|MakeRotator (* (Utilities|Time|GetTimeSeconds) 1e+03) (.Pitch (Math|Vector|GetYawPitchfromVector _returnvalue)) (.Yaw (Math|Vector|GetYawPitchfromVector _returnvalue))) false false)
  (|CallParentFunction DeltaSeconds)
  (if (Math|Boolean|ANDBoolean (< (.Z (Math|Vector|BreakVector (Transformation|GetWorldLocation (Variables|Default|GetSplashRadius)))) (Variables|Default|GetSubmunitionSplitAltitude)) (not (Variables|Default|GethasSplit)) (< (.Z (Math|Vector|BreakVector _returnvalue)) (Variables|Default|GetSubmunitionsSplitVerticalVelocityRequirement)))
    (CallFunction|SubmunitionSplit)))

(fn ConstructionScript
  (|CallParentFunction))

(fn SubmunitionSplit
  (bind _staticmesh (Variables|Default|GetStaticMesh))
  (Utilities|FlowControl|Sequence
    (:then_0
      (for _index (range 0 (Variables|Default|GetNumber%20of%20submunitions))
        (bind _returnvalue (Game|SpawnActorfromClass (Variables|Default|GetSubmunitionsClass) (Math|Transform|MakeTransform (Transformation|GetWorldLocation (Variables|Default|GetSplashRadius)) (Math|Rotator|MakeRotfromXZ (Math|Vector|ProjectVectorontoPlane (Math|Random|RandomUnitVector) (Math|Vector|GetForwardVector _staticmesh)) (Math|Vector|GetUpVector _staticmesh))) "AlwaysSpawn" 0 (Variables|Default|GetSubmunitionsEjectionSpeed) 2e+01 4e+04 1e+04 (Variables|Default|GetPlayerOwner) (Variables|Default|GetInstigator)))
        ;[1 1 1] Inherit velocity, plus its own speed
        (Utilities|IsValid _returnvalue
          (:Is%20Valid
            (bind _returnvalue_2 (Physics|GetPhysicsLinearVelocity (Variables|Default|GetStaticMesh) "None"))
            (Physics|SetPhysicsLinearVelocity (Variables|/Game/Blueprints/Abilities/Projectile_Base.Projectile_Base_C|GetStaticMesh _returnvalue) (+ (* (Transformation|GetActorForwardVector _returnvalue) (* (Variables|Default|GetSubmunitionsEjectionSpeed) (Math|Random|RandomFloat))) _returnvalue_2) false "None")))))
    (:then_1
      (Variables|Default|SethasSplit true)
      (Audio|PlaySound2D "/Game/Audio/Sound/Impact.Impact" 1.0 1.0 0.0 0 0))
    (:then_2
      (CallFunction|OnExpire))
    (:then_3
      (return))))