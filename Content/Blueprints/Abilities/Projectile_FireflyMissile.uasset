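; Heat-seeking missile projectile that picks the nearest visible opposing mech within a forward cone until tracking starts after a delay.
; Tick aligns the physics-driven mesh to its velocity, steering with sideways acceleration scaled by the target's radiator temperature, plus timed forward boost while tracking.
; Impact spawns effects and sound, applies radial damage and detaches the Niagara trail.
; Expiry kills maneuvering and trail, pushing the missile downward before delayed parent cleanup.
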(event EventBeginPlay
  (Utilities|FlowControl|Delay (Variables|Default|GetTrackingDelay))
  (Variables|Default|SetisTracking true)
  (bind _returnvalue (Niagara|SpawnSystemAttached "/Game/VFX/NS_MissileTrail.NS_MissileTrail" (Variables|Default|GetStaticMesh) "None" "0, 0, 0" "0, 0, 0" "SnapToTarget" true true "AutoRelease"))
  (Variables|Default|SetTrail _returnvalue)
  (Utilities|FlowControl|Delay (Variables|Default|GetBoostDelay))
  (Variables|Default|SetisBoosting true))

(event EventTick
  (params (DeltaSeconds :type Float%20%28single-precision%29))
  (bind _staticmesh (Variables|Default|GetStaticMesh))
  (bind _staticmesh_2 (Variables|Default|GetStaticMesh))
  (bind _returnvalue (Math|Vector|GetForwardVector _staticmesh_2))
  (bind _returnvalue_2 (Physics|GetPhysicsLinearVelocity _staticmesh "None"))
  (Transformation|SetWorldRotation _staticmesh (Math|Rotator|MakeRotator 0.0 (.Pitch (Math|Vector|GetYawPitchfromVector _returnvalue_2)) (.Yaw (Math|Vector|GetYawPitchfromVector _returnvalue_2))) false false)
  (|CallParentFunction DeltaSeconds)
  (if (Variables|Default|GetisTracking)
    (Utilities|IsValid (Variables|Default|GetTarget)
      (:Is%20Valid
        ;[1 1 1] Comment
        (if (Rendering|IsVisible (Variables|/Game/Blueprints/Mech_Pawn.Mech_Pawn_C|GetRoot (Variables|Default|GetTarget)))
          (bind _temppercent (Default|GetTempPercent (Variables|/Game/Blueprints/Mech_Pawn.Mech_Pawn_C|GetMechRadiator (Variables|Default|GetTarget))))
          (bind _output_get (Variables|Default|SetBoost%20Time (- (Variables|Default|GetBoost%20Time) (Utilities|Time|GetWorldDeltaSeconds))))
          (bind _output_get_2 (Variables|Default|SetisBoosting (> _output_get 0.0)))
          (Physics|AddForce (Variables|Default|GetStaticMesh) (+ (Math|Vector|ProjectVectorontoPlane (* (Math|Vector|Normalize (- (Transformation|GetWorldLocation (Variables|/Script/Engine.Actor|GetRootComponent (Variables|Default|GetTarget))) (Transformation|GetActorLocation))) (Math|Float|Lerp (Variables|Default|GetManeuver%20Accel%20Min) (Variables|Default|GetManeuver%20Accel%20Max) _temppercent)) _returnvalue) (* _returnvalue (Math|Float|SelectFloat (Variables|Default|GetBoost%20Accel) 0.0 _output_get_2))) "None" true)
          (else
            (Variables|Default|SetTarget 0)))))
    (else
      (bind _outactors (Actor|GetAllActorsOfClass "/Game/Blueprints/Mech_Pawn.Mech_Pawn_C"))
      (CallFunction|FindNearestTargetonOpposingTeam _outactors (Variables|Default|GetTarget%20Acquisition%20Cone%20Half%20Angle)))))

(event EventOnExpire
  (Variables|Default|SetManeuver%20Accel%20Max 0.0)
  (Variables|Default|SetManeuver%20Accel%20Min 0.0)
  (Components|Activation|Deactivate (Variables|Default|GetTrail))
  (Physics|AddForce (Variables|Default|GetStaticMesh) "0, 0,-2000.000000" "None" true)
  (Utilities|FlowControl|Delay 1e+01)
  (|CallParentFunction))

(event Collision|EventHit
  (params (MyComp :type Primitive%20Component%20Object%20Reference) (Other :type Actor%20Object%20Reference) (OtherComp :type Primitive%20Component%20Object%20Reference) (bSelfMoved :type Boolean) (HitLocation :type Vector :default "0, 0, 0") (HitNormal :type Vector :default "0, 0, 0") (NormalImpulse :type Vector :default "0, 0, 0") (Hit :type Hit%20Result%20Structure%20%28by%20ref%29))
  (|CallParentFunction MyComp Other OtherComp bSelfMoved HitLocation HitNormal NormalImpulse Hit))

(event Collision|EventActorBeginOverlap
  (params (OtherActor :type Actor%20Object%20Reference))
  (|CallParentFunction OtherActor))

(fn ConstructionScript
  (|CallParentFunction))

(fn FindNearestTargetonOpposingTeam
  (params (Array :type Array%20of%20Mech%20Pawn%20Object%20References) (TargetAcquisitionConeHalfAngle :type Float%20%28single-precision%29))
  (Variables|Default|SetTarget 0)
  (LocalVariables|SetShortestDistance 3.1366339951612396e+18)
  (for _array_element Array
    (if (Rendering|IsVisible (Variables|/Game/Blueprints/Mech_Pawn.Mech_Pawn_C|GetRoot _array_element))
      (if (!= (Variables|/Game/Blueprints/Mech_Pawn.Mech_Pawn_C|GetTeam _array_element) (Variables|Default|GetTeam))
        (if (< (Math|Vector|VectorLengthSquared (- (Transformation|GetActorLocation _array_element) (Transformation|GetActorLocation))) (LocalVariables|GetShortestDistance))
          (if true
            (if (<= (Class|KismetMathLibrary|DegAcos (Class|KismetMathLibrary|VectorCosineAngle2D (- (Transformation|GetActorLocation _array_element) (Transformation|GetActorLocation)) (Math|Vector|GetForwardVector (Variables|Default|GetStaticMesh)))) TargetAcquisitionConeHalfAngle)
              (LocalVariables|SetShortestDistance (Math|Vector|VectorLengthSquared (- (Transformation|GetActorLocation _array_element) (Transformation|GetActorLocation))) :!label _label)
              (Variables|Default|SetTarget _array_element))
            (else
              (goto _label)))))))
  (return))

(fn OnHitTarget
  (params (hit%20info :type Hit%20Result%20Structure%20%28by%20ref%29))
  (bind _explosionorigin (Variables|Default|GetExplosionOrigin))
  (bind _trail (Variables|Default|GetTrail))
  (bind _returnvalue (Transformation|GetWorldLocation _explosionorigin))
  (Utilities|FlowControl|Sequence
    (:then_0
      (Niagara|SpawnSystematLocation (Variables|Default|GetHit%20FX) _returnvalue (Math|Rotator|MakeRotfromX (Math|Vector|GetForwardVector (Variables|Default|GetStaticMesh))) "1.000000,1.000000,1.000000" true true "AutoRelease")
      (CallFunction|PlaySoundatLocationwithVariance (Variables|Default|GetImpact%20Sound) _returnvalue 1.0 0.15))
    (:then_1
      (Game|Damage|ApplyRadialDamage (Variables|Default|GetAttack) _returnvalue (Variables|Default|GetDamage%20Radius) "/Script/Engine.DamageType" 0 (Variables|Default|GetPlayerOwner) (Game|GetInstigatorController) true "ECC_GameTraceChannel6"))
    (:then_2
      (Utilities|IsValid _trail
        (:Is%20Valid
          (Transformation|DetachFromComponent _trail "KeepWorld" "KeepWorld" "KeepWorld" true))
        (:Is%20Not%20Valid
          _))
      (Actor|DestroyActor)
      (return))))