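; Chain gun ability for a mech, a child Blueprint that adds shell-casing and heat visuals to inherited weapon logic.
; The Casings particle component starts at zero spawn rate, switches to the inverse of Cooldown on activation and returns to zero when cooldown finishes, matching ejection to fire rate.
; Tick updates a heat material parameter every frame, while Fire only calls the parent.
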(event EventBeginPlay
  (|CallParentFunction)
  (Utilities|IsValid (Variables|Default|GetMechOwner)
    (:Is%20Valid
      (Components|Activation|Activate (Variables|Default|GetCasings) true)
      (Effects|Components|ParticleSystem|SetFloatParameter (Variables|Default|GetCasings) "CasingSpawnRate" 0.0))))

(event Collision|EventActorBeginOverlap
  (params (OtherActor :type Actor%20Object%20Reference))
  (|CallParentFunction OtherActor) ; This node is disabled and will not be called.\nDrag off pins to build functionality.
)

(event EventTick
  (params (DeltaSeconds :type Float%20%28single-precision%29))
  (|CallParentFunction DeltaSeconds)
  (CallFunction|SetHeatMaterialParameter))

(event EventOnCooldownFinish
  (|CallParentFunction)
  (Effects|Components|ParticleSystem|SetFloatParameter (Variables|Default|GetCasings) "CasingSpawnRate" 0.0))

(event EventOnActivate
  (|CallParentFunction)
  (Effects|Components|ParticleSystem|SetFloatParameter (Variables|Default|GetCasings) "CasingSpawnRate" (/ 1.0 (Variables|Default|GetCooldown))))

(fn ConstructionScript
  (|CallParentFunction))

(fn Fire
  (|CallParentFunction))