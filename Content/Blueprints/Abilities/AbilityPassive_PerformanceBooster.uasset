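; Passive mech ability that boosts the owning mech's mobility when equipped.
; OnEquip adds bonus variables to the movement component's static top speed and acceleration multipliers, and to the aiming component's torso rotation speed multiplier.
; The bonuses stack additively onto existing multipliers, and this Blueprint has no logic to remove them.
; The activation, cooldown, deactivation and tick events are empty.
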(event Custom|OnActivate)

(event Custom|OnCooldownFinish)

(event Custom|OnDeactivate)

(event EventBeginPlay)

(event Collision|EventActorBeginOverlap
  (params (OtherActor :type Actor%20Object%20Reference)))

(event EventTick
  (params (DeltaSeconds :type Float%20%28single-precision%29)))

(fn ConstructionScript)

(fn OnEquip
  (bind _mechowner (Variables|Default|GetMechOwner))
  (bind _mechmovementcomponent (Variables|/Game/Blueprints/Mech_Pawn.Mech_Pawn_C|GetMechMovementComponent _mechowner))
  (bind _mechaimingcomponent (Variables|/Game/Blueprints/Mech_Pawn.Mech_Pawn_C|GetMechAimingComponent _mechowner))
  (Variables|/Game/Blueprints/Components/MechMovementComponent.MechMovementComponent_C|SetSpeedMaxMultiplierStatic _mechmovementcomponent (+ (Variables|/Game/Blueprints/Components/MechMovementComponent.MechMovementComponent_C|GetSpeedMaxMultiplierStatic _mechmovementcomponent) (Variables|Default|GetTopSpeedBonus)))
  (Variables|/Game/Blueprints/Components/MechMovementComponent.MechMovementComponent_C|SetAccelerationMultiplier _mechmovementcomponent (+ (Variables|/Game/Blueprints/Components/MechMovementComponent.MechMovementComponent_C|GetAccelerationMultiplier _mechmovementcomponent) (Variables|Default|GetAccelerationBonus)))
  (Variables|/Game/Blueprints/Components/MechAimingComponent.MechAimingComponent_C|SetTorsoRotationSpeedMultiplier _mechaimingcomponent (+ (Variables|Default|GetTurnrateBonus) (Variables|/Game/Blueprints/Components/MechAimingComponent.MechAimingComponent_C|GetTorsoRotationSpeedMultiplier _mechaimingcomponent))))