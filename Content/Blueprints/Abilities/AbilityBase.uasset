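; Base Blueprint for mech abilities, with empty equip and unequip hooks and a construction-time check that the AbilityID has a data table row.
; Activation starts the cooldown timer, adds heat to the owning mech's radiator and fires OnActivate.
; Tick counts the timer down and raises OnCooldownFinish at expiry.
; Dynamic materials darken during cooldown via a DoOnce gate, and a helper can feed radiator temperature into the last material.
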(event Custom|OnActivate
  (Utilities|FlowControl|DoOnce false
    (:Completed
      (Utilities|SetCooldownColorMultiply))))

(event Custom|OnCooldownFinish
  (Utilities|ResetCooldownColorMultiply)
  (Utilities|FlowControl|DoOnce false) ; enters at Reset
)

(event Custom|OnDeactivate)

(event EventBeginPlay
  (bind _dynamic_materials (CallFunction|MakeMaterialsDynamic (Variables|Components|GetStaticMesh)))
  (Variables|Default|SetDynamic%20Materials _dynamic_materials))

(event Collision|EventActorBeginOverlap
  (params (OtherActor :type Actor%20Object%20Reference)))

(event EventTick
  (params (DeltaSeconds :type Float%20%28single-precision%29))
  (CallFunction|TickCooldownTimers DeltaSeconds))

(fn ConstructionScript
  (bind _abilityid (Variables|Default|GetAbilityID))
  (bind _returnvalue (Utilities|String|EnumtoString _abilityid))
  ;[0.15 0.15 0.15 0.5] Verify Ability is set up correctly
  (Utilities|GetDataTableRow "/Game/Blueprints/Abilities/AbilityTable.AbilityTable" (Utilities|String|StringToName _returnvalue)
    (:RowNotFound
      (Utilities|Debugging|RaiseScriptError (Utilities|String|BuildString(Name) _returnvalue ": Forgot to set Gear Enum or missing Gear entry in Table: " (Utilities|String|StringToName _returnvalue) "")))))

(fn OnEquip)

(fn OnUnequip)

(fn ActivateAbility
  (Variables|Gameplay|SetCooldownTimer (Variables|Gameplay|GetCooldown))
  (Default|AddHeat (Variables|/Game/Blueprints/Mech_Pawn.Mech_Pawn_C|GetMechRadiator (Variables|Gameplay|GetMechOwner)) (Variables|Gameplay|GetHeatGeneration))
  (CallFunction|OnActivate))

(fn TickCooldownTimers
  (params (DeltaTime :type Float%20%28double-precision%29))
  (Variables|Gameplay|SetCooldownTimer (- (Variables|Gameplay|GetCooldownTimer) DeltaTime))
  (Utilities|FlowControl|Sequence
    (:then_0
      (if (< (Variables|Gameplay|GetCooldownTimer) 0.0)
        (if (Variables|Gameplay|GetOnCooldown)
          (Variables|Gameplay|SetCooldownTimer 0.0)
          (Variables|Gameplay|SetOnCooldown false)
          (CallFunction|OnCooldownFinish))
        (elif (> (Variables|Gameplay|GetCooldown) 0.0)
          (Variables|Gameplay|SetOnCooldown true))))))

(fn DeactivateAbility
  (CallFunction|OnDeactivate))

(fn GetCooldownProgressPercentage
  (return (Math|Float|MapRangeClamped (Variables|Gameplay|GetCooldownTimer) (Variables|Gameplay|GetCooldown) 0.0 0.0 1.0)))

(fn SetHeatMaterialParameter
  (bind _dynamic_materials (Variables|Default|GetDynamic%20Materials))
  (bind _mechowner (Variables|Gameplay|GetMechOwner))
  (Utilities|IsValid _mechowner
    (:Is%20Valid
      (bind _temppercent (Default|GetTempPercent (Variables|/Game/Blueprints/Mech_Pawn.Mech_Pawn_C|GetMechRadiator _mechowner)))
      (Rendering|Material|SetScalarParameterValue (Utilities|Array|Get(acopy) _dynamic_materials (Utilities|Array|LastIndex _dynamic_materials)) "ParamHeat" _temppercent :!class /Script/Engine.MaterialInstanceDynamic))))