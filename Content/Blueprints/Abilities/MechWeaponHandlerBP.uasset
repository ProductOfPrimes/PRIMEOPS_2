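; Weapon handler for a mech that manages a four-slot loadout of arm and shoulder abilities.
; DefineStartingLoadout maps gear choices to weapon classes, then Init spawns each one, stores it by slot and attaches it to its skeletal mesh socket.
; FireWeapon activates a slot's ability unless it is on cooldown or the owner's MechRadiator is overheated.
; AddHeat keeps a separate heat value and overheat flag that firing ignores; Equip is empty.
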(event EventBeginPlay)

(event EventTick
  (params (DeltaSeconds :type Float%20%28single-precision%29)))

(fn AddHeat
  (params (heat :type Float%20%28single-precision%29))
  (bind _heatpercentage (CallFunction|GetHeatPercentage))
  (LocalVariables|SetPreviousHeatPercentage _heatpercentage)
  (bind _output_get (Variables|Default|SetHeat (Math|Float|Max(Float) (+ heat (Variables|Default|GetHeat)) 0.0)))
  (bind _heatpercentage_2 (CallFunction|GetHeatPercentage))
  (LocalVariables|SetHeatPercentage _heatpercentage_2)
  (if (and (>= _output_get (Variables|Default|GetMaxHeat)) (not (Variables|Default|GetIsOverHeated))) ; Trigger Overheat
    (Variables|Default|SetIsOverHeated true)
    (elif (and (> (LocalVariables|GetHeatPercentage) (Variables|Default|GetHeatWarningThreshold)) (<= (LocalVariables|GetPreviousHeatPercentage) (Variables|Default|GetHeatWarningThreshold)))
      _)))

(fn GetHeatPercentage
  (return (/ (Variables|Default|GetHeat) (Variables|Default|GetMaxHeat))))

(fn Equip)

(fn AddAbility
  (params (Slot :type GearSlot%20Enum :default "L_ARM") (Ability :type Ability%20Base%20Object%20Reference))
  (Utilities|Array|SetArrayElem (Variables|Default|GetLoadout) (Math|Conversions|ToInteger(Byte) Slot) Ability)
  (Variables|/Game/Blueprints/Abilities/AbilityBase.AbilityBase_C|SetMechOwner Ability (Variables|Default|GetMech%20Owner))
  (if (Utilities|IsValid (Variables|Default|GetMech%20Owner))
    _))

(fn FireWeapon
  (params (slot :type GearSlot%20Enum :default "L_ARM"))
  (bind _returnvalue (Math|Conversions|ToInteger(Byte) slot))
  (bind _loadout (Variables|Default|GetLoadout))
  (bind _output (Utilities|Array|Get(acopy) _loadout _returnvalue))
  (if (not (Variables|/Game/Blueprints/MechRadiator.MechRadiator_C|GetOverheated (Variables|/Game/Blueprints/Mech_Pawn.Mech_Pawn_C|GetMechRadiator (Variables|Default|GetMech%20Owner))))
    (Utilities|IsValid _output
      (:Is%20Valid
        (if (not (Variables|/Game/Blueprints/Abilities/AbilityBase.AbilityBase_C|GetOnCooldown _output))
          (Default|ActivateAbility _output))))))

(fn Init
  (bind _startingloadout (Variables|Default|GetStartingLoadout))
  (bind _mech_owner (Variables|Default|GetMech%20Owner))
  (bind _returnvalue (Actor|GetComponentbyClass _mech_owner "/Script/Engine.SkeletalMeshComponent"))
  (Utilities|FlowControl|Sequence
    (:then_0
      (bind _asability_base (Utilities|Casting|CastToAbilityBaseClass (Utilities|Array|Get(acopy) _startingloadout)))
      (bind _returnvalue_2 (Game|SpawnActorfromClass _asability_base (Transformation|GetSocketTransform _returnvalue "LeftHand Socket" "RTS_World") "AlwaysSpawn" 0 _mech_owner 0))
      (CallFunction|AddAbility "L_ARM" _returnvalue_2)
      (Transformation|AttachComponentToComponent _returnvalue_2 _returnvalue "LeftHand Socket" "KeepWorld" "KeepWorld" "KeepWorld" true))
    (:then_1
      (bind _asability_base_2 (Utilities|Casting|CastToAbilityBaseClass (Utilities|Array|Get(acopy) _startingloadout 1)))
      (bind _returnvalue_3 (Game|SpawnActorfromClass _asability_base_2 (Transformation|GetSocketTransform _returnvalue "LeftShoulder Socket" "RTS_World") "AlwaysSpawn" 0 _mech_owner 0))
      (CallFunction|AddAbility "L_SHD" _returnvalue_3)
      (Transformation|AttachComponentToComponent _returnvalue_3 _returnvalue "LeftShoulder Socket" "KeepWorld" "KeepWorld" "KeepWorld" true))
    (:then_2
      (bind _asability_base_3 (Utilities|Casting|CastToAbilityBaseClass (Utilities|Array|Get(acopy) _startingloadout 2)))
      (bind _returnvalue_4 (Game|SpawnActorfromClass _asability_base_3 (Transformation|GetSocketTransform _returnvalue "RightShoulder Socket" "RTS_World") "AlwaysSpawn" 0 _mech_owner 0))
      (CallFunction|AddAbility "R_SHD" _returnvalue_4)
      (Transformation|AttachComponentToComponent _returnvalue_4 _returnvalue "RightShoulder Socket" "KeepWorld" "KeepWorld" "KeepWorld" true))
    (:then_3
      (bind _asability_base_4 (Utilities|Casting|CastToAbilityBaseClass (Utilities|Array|Get(acopy) _startingloadout 3)))
      (bind _returnvalue_5 (Game|SpawnActorfromClass _asability_base_4 (Transformation|GetSocketTransform _returnvalue "RightHand Socket" "RTS_World") "AlwaysSpawn" 0 _mech_owner 0))
      (CallFunction|AddAbility "R_ARM" _returnvalue_5)
      (Transformation|AttachComponentToComponent _returnvalue_5 _returnvalue "RightHand Socket" "KeepWorld" "KeepWorld" "KeepWorld" true))))

(fn DefineStartingLoadout
  (params (Abilities :type Array%20of%20Abilities%20Enums :default "NewEnumerator1"))
  (for (_array_element _array_index) Abilities
    (switch Utilities|FlowControl|Switch|SwitchonAbilities _array_element
      (:NewEnumerator1
        (Utilities|Array|SetArrayElem (Variables|Default|GetStartingLoadout) _array_index "/Game/Blueprints/Abilities/Sniper.Sniper_C"))
      (:NewEnumerator2
        (Utilities|Array|SetArrayElem (Variables|Default|GetStartingLoadout) _array_index "/Game/Blueprints/Abilities/Shotgun.Shotgun_C"))
      (:NewEnumerator5
        (Utilities|Array|SetArrayElem (Variables|Default|GetStartingLoadout) _array_index "/Game/Blueprints/Abilities/MachineGun.MachineGun_C"))
      (:NewEnumerator8
        (Utilities|Array|SetArrayElem (Variables|Default|GetStartingLoadout) _array_index "/Game/Blueprints/Abilities/GrenadeLauncher.GrenadeLauncher_C"))))
  (CallFunction|Init))