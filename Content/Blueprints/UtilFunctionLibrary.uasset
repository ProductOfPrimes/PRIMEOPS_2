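; A Blueprint function library of shared gameplay helpers for a mech game with teams and abilities.
; It plays sounds with random pitch variance, generates time-based sine and square wave floats, wraps indices and creates dynamic materials for meshes.
; Team and ability data come from data table rows keyed by enum name, with missing rows reported.
; Team colors are converted from bytes to float vectors and written into armor material parameters.
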(fn PlaySoundatLocationwithVariance
  (params (Sound :type Sound%20Base%20Object%20Reference) (Location :type Vector%20%28by%20ref%29) (PitchBase :type Float%20%28double-precision%29) (PitchVariance :type Float%20%28double-precision%29))
  (Audio|PlaySoundatLocation 0 Sound Location "0, 0, 0" 1.0 (+ PitchBase (Math|Random|RandomFloatinRange (* PitchVariance -1.0) PitchVariance)) 0.0 0 0 0 0)
  (return))

(fn PeriodicFloat
  (params (Frequency :type Float%20%28double-precision%29) (Amplitude :type Float%20%28double-precision%29) (offset :type Float%20%28double-precision%29))
  (return (+ (* (Math|Trig|Sin(Radians) (* (Utilities|Time|GetTimeSeconds) Frequency 6.28)) Amplitude) offset)))

(fn PeriodicFloatSquare
  (params (Frequency :type Float%20%28double-precision%29) (Amplitude :type Float%20%28double-precision%29) (offset :type Float%20%28double-precision%29))
  (return (+ (Math|Float|Clamp(Float) (* (Math|Trig|Sin(Radians) (* (Utilities|Time|GetTimeSeconds) Frequency 6.28)) 999999995904.0) (* Amplitude -1.0) Amplitude) offset)))

(fn PlayRandomSoundatLocationwithVariance
  (params (Sound :type Array%20of%20Sound%20Base%20Object%20References) (Location :type Vector%20%28by%20ref%29) (PitchBase :type Float%20%28double-precision%29) (PitchVariance :type Float%20%28double-precision%29))
  (Audio|PlaySoundatLocation 0 (Utilities|Array|Get(acopy) Sound (Math|Random|RandomInteger (Utilities|Array|Length Sound))) Location "0, 0, 0" 1.0 (+ PitchBase (Math|Random|RandomFloatinRange (* PitchVariance -1.0) PitchVariance)) 0.0 0 0 0 0)
  (return))

(fn Repeat
  (params (Input :type Integer) (Length :type Integer))
  (if (>= Input Length)
    (return 0)
    (elif (> Input -1)
      (return Input)
      (else
        (return (- Length 1))))))

(fn MakeMaterialsDynamic
  (params (Mesh :type Mesh%20Component%20Object%20Reference%20%28by%20ref%29))
  (bind _materials (LocalVariables|Getmaterials))
  (for (_array_element _array_index) (Rendering|Material|GetMaterials Mesh)
    (bind _returnvalue (Rendering|Material|CreateDynamicMaterialInstance 0 _array_element "None" :!class /Script/Engine.KismetMaterialLibrary))
    (Rendering|Material|SetMaterial Mesh _array_index _returnvalue)
    (Utilities|Array|Add _materials _returnvalue))
  (return _materials))

(fn UpdateMaterialParamstoTeamColor
  (params (Mesh :type Array%20of%20Mesh%20Component%20Object%20References) (Team :type Team%20Enum :default "NewEnumerator0"))
  (bind (_main_color _sub_color) (CallFunction|GetTeamColor 0 Team))
  (bind _returnvalue (CallFunction|ByteColortoFloatVector _main_color))
  (bind _returnvalue_2 (CallFunction|ByteColortoFloatVector _sub_color))
  (for _array_element Mesh
    (Rendering|Material|SetVectorParameterValueonMaterials _array_element "ArmorColorMain" _returnvalue)
    (Rendering|Material|SetVectorParameterValueonMaterials _array_element "ArmorColorSub" _returnvalue_2)))

(fn ByteColortoFloatVector
  (params (Color :type Color%20Structure%20%28by%20ref%29))
  (bind (_b _g _r) (Math|Color|BreakColor Color))
  (bind _returnvalue (Math|Float|MakeLiteralFloat 0.003922))
  (return (Math|Vector|MakeVector (* (Math|Conversions|ToFloat(Byte) _r) _returnvalue) (* (Math|Conversions|ToFloat(Byte) _g) _returnvalue) (* (Math|Conversions|ToFloat(Byte) _b) _returnvalue))))

(fn GetTeamColor
  (params (Enumerator :type Team%20Enum :default "NewEnumerator0"))
  (bind _returnvalue (Utilities|String|EnumtoString Enumerator))
  (bind _returnvalue_2 (Utilities|String|StringToName _returnvalue))
  (bind _returnvalue_3 (Utilities|GetDataTableRow "/Game/Blueprints/TeamTable.TeamTable" _returnvalue_2)
    (:then
      _)
    (:RowNotFound
      (Development|PrintString 0 (Utilities|String|Append "Could not find team color for: " (Utilities|String|ToString(Name) _returnvalue_2)))))
  (return (.Color (Utilities|Struct|BreakTeamInfo _returnvalue_3)) (.SubColor (Utilities|Struct|BreakTeamInfo _returnvalue_3))))

(fn GetMechName
  (params (Mech :type Mech%20Pawn%20Object%20Reference))
  (return (Utilities|Text|FormatText "P{PlayerNumber}" (+ (Variables|/Game/Blueprints/Mech_Pawn.Mech_Pawn_C|GetPlayerInt Mech) 1))))

(fn GetAbilityInfo
  (params (Ability :type Ability%20Base%20Object%20Reference))
  (bind _abilityid (Variables|/Game/Blueprints/Abilities/AbilityBase.AbilityBase_C|GetAbilityID Ability))
  (bind _returnvalue (Utilities|String|EnumtoString _abilityid))
  (bind _returnvalue_2 (Utilities|String|StringToName _returnvalue))
  (bind _returnvalue_3 (Utilities|GetDataTableRow "/Game/Blueprints/Abilities/AbilityTable.AbilityTable" _returnvalue_2)
    (:then
      (return _returnvalue_3))
    (:RowNotFound
      (Utilities|Debugging|RaiseScriptError (Utilities|String|BuildString(Name) (Utilities|GetDisplayName Ability) ": Missing Gear from table with name: " _returnvalue_2 "")))))