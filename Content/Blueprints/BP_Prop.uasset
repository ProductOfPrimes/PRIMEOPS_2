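; BP_Prop is a destructible prop that breaks on any damage, including damage it applies to itself when an actor overlaps it.
; On BeginPlay, props with a DestroyedMesh hide it and add an enlarged, bounds-sized collision box on a custom channel.
; Damage plays a randomly pitched sound and dust effect, hides MainMesh, then reveals DestroyedMesh and removes the box, or destroys the actor if no such mesh exists.
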(event Collision|EventActorBeginOverlap
  (params (OtherActor :type Actor%20Object%20Reference))
  (Game|Damage|ApplyDamage self 1.0 0 OtherActor "/Engine/EngineDamageTypes/DmgTypeBP_Environmental.DmgTypeBP_Environmental_C"))

(event EventBeginPlay
  (bind _boxextent (Collision|GetActorBounds false true))
  (bind _destroyedmesh (Variables|Default|GetDestroyedMesh))
  (Utilities|IsValid _destroyedmesh
    (:Is%20Valid
      (Rendering|SetVisibility _destroyedmesh false true)
      (bind _returnvalue (AddComponent|AddBoxComponent false (Math|Conversions|ToTransform(Vector) (* _boxextent "0, 0,1.000000"))))
      (bind _output_get (Variables|Default|SetBoxCollision _returnvalue))
      (Collision|SetCollisionObjectType _output_get "ECC_GameTraceChannel1")
      (Components|Box|SetBoxExtent _output_get (* _boxextent 1.8) true))))

(event Game|Damage|EventAnyDamage
  (params (Damage :type Float%20%28single-precision%29) (DamageType :type Damage%20Type%20Object%20Reference) (InstigatedBy :type Controller%20Object%20Reference) (DamageCauser :type Actor%20Object%20Reference))
  (bind _boxcollision (Variables|Default|GetBoxCollision))
  (bind _destroyedmesh (Variables|Default|GetDestroyedMesh))
  (Audio|PlaySoundatLocation "/Game/Audio/Sound/PlayerHit.PlayerHit" (Transformation|GetActorLocation) "0, 0, 0" 1.0 (Utilities|RandomFloatwithVariance 1.0 0.5) 0.0 0 0 0 0)
  (Niagara|SpawnSystematLocation "/Game/VFX/NS_BuildingDustSmall.NS_BuildingDustSmall" (Transformation|GetWorldLocation (Variables|Default|GetMainMesh)))
  (Rendering|SetVisibility (Variables|Default|GetMainMesh) false true)
  (Utilities|IsValid _destroyedmesh
    (:Is%20Valid
      ;[1 1 1] Replace model
      (Rendering|SetVisibility _destroyedmesh true true)
      (Utilities|IsValid _boxcollision
        (:Is%20Valid
          (Components|DestroyComponent _boxcollision))))
    (:Is%20Not%20Valid
      ;[1 1 1] Destroy Actor
      (Actor|DestroyActor))))

(fn ConstructionScript)

(fn ResetPhysicsInvuln)