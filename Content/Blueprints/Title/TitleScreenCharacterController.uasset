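; Title screen controller that holds a reference to the title widget and provides keyboard shortcuts for inspecting and wiping user profiles.
; Pressing D prints every key of the ProfileController's UserProfiles map, and pressing X calls ClearProfiles on that actor.
; Both handlers look up the ProfileController with GetActorOfClass on each press, while Init only stores the passed-in TitleWidget.
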(event EventBeginPlay)

(event EventTick
  (params (DeltaSeconds :type Float%20%28single-precision%29)))

(event Input|KeyboardEvents|D
  (params (Key :type Key%20Structure :default "None"))
  (:Pressed
    (Development|PrintString "Printing Profile Names")
    (bind _returnvalue (Actor|GetActorOfClass "/Game/Blueprints/ControlMapping/ProfileController.ProfileController_C"))
    (bind _keys (Utilities|Map|Keys (Variables|/Game/Blueprints/ControlMapping/ProfileController.ProfileController_C|GetUserProfiles _returnvalue)))
    (for _array_element _keys
      (Development|PrintString _array_element))))

(event Input|KeyboardEvents|X
  (params (Key :type Key%20Structure :default "None"))
  (:Pressed
    (bind _returnvalue (Actor|GetActorOfClass "/Game/Blueprints/ControlMapping/ProfileController.ProfileController_C"))
    (Default|ClearProfiles _returnvalue)))

(fn ConstructionScript)

(fn Init
  (params (TitleWidget :type Main%20Title%20Widget%20Object%20Reference))
  (Variables|Default|SetTitleWidget TitleWidget)
  (return))