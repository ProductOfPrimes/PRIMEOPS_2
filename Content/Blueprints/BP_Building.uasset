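; Destructible building actor that takes damage, visibly degrades and crumbles when destroyed.
; Construction script fits the Box to the actor bounds and loads health and momentum threshold from a data table row keyed by Size.
; Damage events trigger dust and HitResponse, which updates LivingActorComponent, shakes, plays sound, darkens dynamic materials by health, and on death sinks and rotates the mesh before destroying the actor.
; Momentum-based collision damage is disconnected.
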(event Game|Damage|EventAnyDamage
  (params (Damage :type Float%20%28single-precision%29) (DamageType :type Damage%20Type%20Object%20Reference) (InstigatedBy :type Controller%20Object%20Reference) (DamageCauser :type Actor%20Object%20Reference))
  (Niagara|ResetSystem (Variables|Default|GetDust%20FX))
  (Utilities|HitResponse Damage))

(event EventBeginPlay
  (bind _mainmesh (Variables|Default|GetMainMesh))
  (CallFunction|MakeMaterialsDynamic (Variables|Default|GetMainMesh))
  (Class|NiagaraFunctionLibrary|OverrideSystemUserVariableStaticMeshComponent (Variables|Default|GetDust%20FX) "System_surface" (Variables|Default|GetMainMesh))
  (Collision|SetCollisionObjectType _mainmesh "ECC_Destructible")
  (Collision|SetCollisionProfileName _mainmesh "Default" false :!class /Script/Engine.PrimitiveComponent)
  (Transformation|SetMobility (Variables|Default|GetMainMesh) "Movable"))

(event Collision|EventHit
  (params (MyComp :type Primitive%20Component%20Object%20Reference) (Other :type Actor%20Object%20Reference) (OtherComp :type Primitive%20Component%20Object%20Reference) (bSelfMoved :type Boolean) (HitLocation :type Vector :default "0, 0, 0") (HitNormal :type Vector :default "0, 0, 0") (NormalImpulse :type Vector :default "0, 0, 0") (Hit :type Hit%20Result%20Structure%20%28by%20ref%29))
  ;[1 1 1] Collision Damage
)

(event Game|Damage|EventPointDamage
  (params (Damage :type Float%20%28single-precision%29) (DamageType :type Damage%20Type%20Object%20Reference) (HitLocation :type Vector :default "0, 0, 0") (HitNormal :type Vector :default "0, 0, 0") (HitComponent :type Primitive%20Component%20Object%20Reference) (BoneName :type Name :default "None") (ShotFromDirection :type Vector :default "0, 0, 0") (InstigatedBy :type Controller%20Object%20Reference) (DamageCauser :type Actor%20Object%20Reference) (HitInfo :type Hit%20Result%20Structure%20%28by%20ref%29))
  (Niagara|SpawnSystematLocation "/Game/VFX/Impacts/NS_ProjectileImpactDust.NS_ProjectileImpactDust" HitLocation (Math|Conversions|RotationFromXVector HitNormal) "1.000000,1.000000,1.000000" true true "AutoRelease")
  (Utilities|HitResponse Damage))

(fn ConstructionScript
  (bind (_origin _boxextent) (Collision|GetActorBounds true true))
  (bind _size (Variables|Default|GetSize))
  (bind _returnvalue (Utilities|String|EnumtoString _size))
  (bind _returnvalue_2 (Utilities|String|StringToName _returnvalue))
  (Variables|Default|SetActor%20Center (* _origin "1.000000,1.000000,0.000000"))
  (bind _output_get (Variables|Default|SetActorBounds _boxextent))
  (Transformation|SetRelativeLocation (Variables|Default|GetBox) (+ "0, 0, 0" (* _output_get "0.500000,-0.500000,0.500000")) false true)
  (Components|Box|SetBoxExtent (Variables|Default|GetBox) _output_get true)
  (bind _returnvalue_3 (Utilities|GetDataTableRow "/Game/Blueprints/Building_Stats_Table.Building_Stats_Table" _returnvalue_2)
    (:then
      (Variables|/Game/Blueprints/LivingActorComponent.LivingActorComponent_C|SetMaxHealth (Variables|Default|GetLivingActorComponent) (.HitPointsMax (Utilities|Struct|BreakBuildingStats _returnvalue_3)))
      (Variables|Default|SetMinimumMomentumToCauseDamage (.MinimumMomentumToDamage (Utilities|Struct|BreakBuildingStats _returnvalue_3))))
    (:RowNotFound
      (Development|PrintString (Utilities|String|BuildString(Name) "" "Building type: " _returnvalue_2 " Not found")))))

(fn ResetPhysicsInvuln
  (Variables|Default|SetPhysicsHittable true))