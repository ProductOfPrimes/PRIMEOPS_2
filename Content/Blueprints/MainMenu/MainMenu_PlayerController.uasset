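; Player controller for the main menu that forwards each local player's gamepad input to the MainMenuHUD.
; Init stores the HUD reference, and each input event calls a matching HUD function tagged with the player's controller ID, so the HUD knows who pressed.
; D-pad, confirm, cancel, start and back drive navigation and screen changes, shoulder and hand inputs pass their key to MenuCustom, and the LookForward axis feeds MenuLook.
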(event EventBeginPlay)

(event EventTick
  (params (DeltaSeconds :type Float%20%28single-precision%29)))

(event Input|ActionEvents|InputActionD-PadRight
  (params (Key :type Key%20Structure :default "None"))
  (:Pressed
    (Default|MenuRight (Variables|Default|GetMainMenuHUD) (Class|GameplayStatics|GetPlayerControllerID self))))

(event Input|ActionEvents|InputActionBack
  (params (Key :type Key%20Structure :default "None"))
  (:Pressed
    (Default|RevertScreens (Variables|Default|GetMainMenuHUD) (Class|GameplayStatics|GetPlayerControllerID self))))

(event Input|ActionEvents|InputActionD-PadDown
  (params (Key :type Key%20Structure :default "None"))
  (:Pressed
    (Default|MenuDown (Variables|Default|GetMainMenuHUD) (Class|GameplayStatics|GetPlayerControllerID self))))

(event Input|ActionEvents|InputActionConfirm
  (params (Key :type Key%20Structure :default "None"))
  (:Pressed
    (Default|MenuConfirm (Variables|Default|GetMainMenuHUD) (Class|GameplayStatics|GetPlayerControllerID self))))

(event Input|ActionEvents|InputActionCancel
  (params (Key :type Key%20Structure :default "None"))
  (:Pressed
    (Default|MenuCancel (Variables|Default|GetMainMenuHUD) (Class|GameplayStatics|GetPlayerControllerID self))))

(event Input|ActionEvents|InputActionStart
  (params (Key :type Key%20Structure :default "None"))
  (:Pressed
    (Default|AdvanceScreens (Variables|Default|GetMainMenuHUD) (Class|GameplayStatics|GetPlayerControllerID self))))

(event Input|ActionEvents|InputActionLeftShoulder
  (params (Key :type Key%20Structure :default "None"))
  (:Pressed
    (Default|MenuCustom (Variables|Default|GetMainMenuHUD) (Class|GameplayStatics|GetPlayerControllerID self) Key)))

(event Input|ActionEvents|InputActionLeftHand
  (params (Key :type Key%20Structure :default "None"))
  (:Pressed
    (Default|MenuCustom (Variables|Default|GetMainMenuHUD) (Class|GameplayStatics|GetPlayerControllerID self) Key)))

(event Input|ActionEvents|InputActionRightHand
  (params (Key :type Key%20Structure :default "None"))
  (:Pressed
    (Default|MenuCustom (Variables|Default|GetMainMenuHUD) (Class|GameplayStatics|GetPlayerControllerID self) Key)))

(event Input|ActionEvents|InputActionD-PadUp
  (params (Key :type Key%20Structure :default "None"))
  (:Pressed
    (Default|MenuUp (Variables|Default|GetMainMenuHUD) (Class|GameplayStatics|GetPlayerControllerID self))))

(event Input|ActionEvents|InputActionD-PadLeft
  (params (Key :type Key%20Structure :default "None"))
  (:Pressed
    (Default|MenuLeft (Variables|Default|GetMainMenuHUD) (Class|GameplayStatics|GetPlayerControllerID self))))

(event Input|AxisEvents|InputAxisMoveForward
  (params (AxisValue :type Float%20%28single-precision%29)))

(event Input|AxisEvents|InputAxisMoveRight
  (params (AxisValue :type Float%20%28single-precision%29)))

(event Input|AxisEvents|InputAxisLookForward
  (params (AxisValue :type Float%20%28single-precision%29))
  (Default|MenuLook (Variables|Default|GetMainMenuHUD) (Class|GameplayStatics|GetPlayerControllerID self) AxisValue))

(event Input|AxisEvents|InputAxisLookRight
  (params (AxisValue :type Float%20%28single-precision%29)))

(event Input|GamepadEvents|GamepadRightShoulder
  (params (Key :type Key%20Structure :default "None"))
  (:Pressed
    (Default|MenuCustom (Variables|Default|GetMainMenuHUD) (Class|GameplayStatics|GetPlayerControllerID self) Key)))

(fn ConstructionScript)

(fn Init
  (params (hud :type HUD%20Main%20Menu%20Object%20Reference%20%28by%20ref%29))
  (Variables|Default|SetMainMenuHUD hud))