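; Shared camera controller that frames all Mech_Pawns in the level, becoming player 0's view target after a startup delay.
; Each tick it measures the largest pairwise mech distance, weighting X more heavily, to set the clamped spring arm length, and lerps a box toward their average position.
; A mech death temporarily changes the zoom interpolation speed.
; GetZoomScale exposes current zoom as a fraction of maximum distance.
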(event Custom|DistanceCheck
  ;[1 1 1] Finds the greatest distance between players
  (bind _outactors (Actor|GetAllActorsOfClass "/Game/Blueprints/Mech_Pawn.Mech_Pawn_C"))
  (if (not (<= (Utilities|Array|Length _outactors) 0))
    (Variables|Maths|SetLongestDistance 0.0)
    (if (not (<= (Utilities|Array|Length _outactors) 1)) ; If there is only a single mech we want to focus on it
      (for _index (range 0 (- (Utilities|Array|Length _outactors) 1))
        (Utilities|IsValid (Utilities|Array|Get(acopy) _outactors _index)
          (:Is%20Valid
            (Variables|Default|SetPawn0 (Utilities|Array|Get(acopy) _outactors _index))
            (for _index_2 (range (+ _index 1) (- (Utilities|Array|Length _outactors) 1))
              (bind _output_get (Variables|Default|SetPawn1 (Utilities|Array|Get(acopy) _outactors _index_2)))
              (Utilities|IsValid _output_get
                (:Is%20Valid
                  (if (> (- (Math|Vector|VectorLength (Math|Vector|MakeVector (* (- (.x (Transformation|GetActorLocation (Variables|Default|GetPawn0))) (.x (Transformation|GetActorLocation (Variables|Default|GetPawn1)))) 1.5) (- (.y (Transformation|GetActorLocation (Variables|Default|GetPawn0))) (.y (Transformation|GetActorLocation (Variables|Default|GetPawn1)))) (- (.z (Transformation|GetActorLocation (Variables|Default|GetPawn0))) (.z (Transformation|GetActorLocation (Variables|Default|GetPawn1)))))) (Variables|Default|Getwtf)) (Variables|Maths|GetLongestDistance))
                    (Variables|Maths|SetLongestDistance (- (Math|Vector|VectorLength (Math|Vector|MakeVector (* (- (.x (Transformation|GetActorLocation (Variables|Default|GetPawn0))) (.x (Transformation|GetActorLocation (Variables|Default|GetPawn1)))) 1.5) (- (.y (Transformation|GetActorLocation (Variables|Default|GetPawn0))) (.y (Transformation|GetActorLocation (Variables|Default|GetPawn1)))) (- (.z (Transformation|GetActorLocation (Variables|Default|GetPawn0))) (.z (Transformation|GetActorLocation (Variables|Default|GetPawn1)))))) (Variables|Default|Getwtf)))))))))))))

(event Custom|Find%20Midpoint
  ;[1 1 1] Find the midpoint between the players. Where the camera should be looking
  (bind _outactors (Actor|GetAllActorsOfClass "/Game/Blueprints/Mech_Pawn.Mech_Pawn_C"))
  (if (not (<= (Utilities|Array|Length _outactors) 0))
    (Variables|Maths|SetMidpoint "0, 0, 0")
    (for _index (range 0 (- (Utilities|Array|Length _outactors) 1))
      (Utilities|IsValid (Utilities|Array|Get(acopy) _outactors _index)
        (:Is%20Valid
          (Variables|Maths|SetMidpoint (+ (Variables|Maths|GetMidpoint) (Transformation|GetActorLocation (Utilities|Array|Get(acopy) _outactors _index)))))))
    (Variables|Maths|SetMidpoint (/ (Variables|Maths|GetMidpoint) (Utilities|Array|Length _outactors)))))

(event Custom|CameraZoom
  (bind _springarm (Variables|Default|GetSpringArm))
  ;[1 1 1] Zoom camera in or out
  (bind _output_get (Variables|/Script/Engine.SpringArmComponent|SetTargetArmLength _springarm (Math|Interpolation|FInterpTo (Variables|/Script/Engine.SpringArmComponent|GetTargetArmLength _springarm) (Math|Float|Max(Float) (Math|Float|Min(Float) (Variables|Maths|GetLongestDistance) (Variables|Maths|GetMaxCameraDistance)) (Variables|Maths|GetMinCameraDistance)) (Variables|Maths|Getdt) (Variables|Maths|GetInterpSpeed))))
  (Variables|Maths|SetCurrentCameraDistance _output_get))

(event Custom|SetCameraLook
  (bind _box (Variables|Default|GetBox))
  ;[1 1 1] Move the look position of the camera
  (Transformation|SetWorldLocation _box (Math|Vector|Lerp(Vector) (Transformation|GetWorldLocation _box) (Variables|Maths|GetMidpoint) 0.05) false true))

(event Custom|Death
  (Utilities|Array|RemoveItem (stale Custom|InitializeMechArray _output_get) (stale Custom|InitializeMechArray _array_element))
  (Variables|Maths|SetInterpSpeed 0.1)
  (Utilities|FlowControl|Delay 7.5)
  (Variables|Maths|SetInterpSpeed 0.0))

(event Custom|InitializeMechArray
  (bind _outactors (Actor|GetAllActorsOfClass "/Game/Blueprints/Mech_Pawn.Mech_Pawn_C"))
  (bind _output_get (Variables|Default|SetMechPawns _outactors))
  (for _array_element _output_get
    (EventDispatchers|BindEventtoOnDeath _array_element (delegate Custom|Death))
    (Game|Player|SetViewTargetwithBlend (Game|GetPlayerController 0) self 0.0 "VTBlend_Linear" 0.0 false)
    (Development|PrintString "Camera Controller Registered player" true true "(R=0.000000,G=0.660000,B=1.000000,A=1.000000)" 9.0)))

(event EventBeginPlay
  (bind _returnvalue (Transformation|GetActorLocation))
  (bind _springarm (Variables|Default|GetSpringArm))
  (bind _returnvalue_2 (Transformation|GetWorldLocation _springarm))
  (Utilities|FlowControl|Sequence
    (:then_0
      (Utilities|FlowControl|Delay 5.0)
      (CallFunction|InitializeMechArray))
    (:then_1
      (Variables|Maths|SetCamXPos (.x _returnvalue_2))
      (Variables|Maths|SetCamYPos (.y _returnvalue_2))
      (Variables|Maths|SetCameraStartPos (Math|Vector|MakeVector (.x _returnvalue) (.y _returnvalue) (.z _returnvalue))))))

(event EventTick
  (params (DeltaSeconds :type Float%20%28single-precision%29))
  (Variables|Maths|Setdt DeltaSeconds)
  (CallFunction|DistanceCheck)
  (CallFunction|FindMidpoint)
  (CallFunction|CameraZoom)
  (CallFunction|SetCameraLook))

(fn ConstructionScript)

(fn GetZoomScale
  (return (/ (Variables|Maths|GetCurrentCameraDistance) (Variables|Maths|GetMaxCameraDistance))))