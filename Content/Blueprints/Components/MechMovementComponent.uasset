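; Physics-based movement component for a mech, driving the owner's primitive body with forces.
; Tick sphere-traces below the capsule for upward-facing terrain, updates grounded state, pulls the body down when off ground, and applies movement acceleration.
; MoveOnGround derives that acceleration from target velocity and a speed-based curve, applies queued knockback, and brakes with friction unless dashing.
; Additive, index-addressed speed modifiers adjust the max speed used to sample the curve.
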(event Custom|OnLeaveGround
  (Variables|Default|SetisGrounded false))

(event Custom|OnTouchGround
  (Variables|Default|SetisGrounded true))

(event EventBeginPlay
  (Variables|Default|SetBodyPrimitive (Actor|GetComponentbyClass (Components|GetOwner) "/Script/Engine.PrimitiveComponent"))
  (EventDispatchers|BindEventtoDispatcheronTouchGround (delegate Custom|OnTouchGround))
  (EventDispatchers|BindEventtoDispatcheronLeaveGround (delegate Custom|OnLeaveGround))
  (CallFunction|UpdateSpeedModifier))

(event EventTick
  (params (DeltaSeconds :type Float%20%28single-precision%29))
  (bind _ascapsule_collision (Utilities|Casting|CastToCapsuleComponent (Variables|Default|GetBodyPrimitive)))
  ;[0.15 0.15 0.15 0.5] Grounded Check
  (bind (_outhit _returnvalue) (Class|KismetSystemLibrary|SphereTraceSinglebyProfile (+ (Transformation|GetWorldLocation _ascapsule_collision) "0, 0,1000.000000") (+ (Transformation|GetWorldLocation _ascapsule_collision) (* "0, 0,-1.000000" (Components|Capsule|GetScaledCapsuleHalfHeight _ascapsule_collision)) "0,0,-100.000000") (* (Components|Capsule|GetScaledCapsuleRadius _ascapsule_collision) 0.5) "BlockTerrain" false 0 "None" true))
  (if (and _returnvalue (> (Math|Vector|DotProduct (.Normal (Collision|BreakHitResult _outhit)) "0, 0,1.000000") 0.5))
    (if (Variables|Default|GetisGrounded)
      _
      (else
        (CallFunction|OnTouchGround)))
    (else
      (if (Variables|Default|GetisGrounded)
        (Default|CallDispatcheronLeaveGround))
      (Physics|AddForce (Variables|Default|GetBodyPrimitive) "0.000000,0.000000,-8000.000000" "None" true) ; To help stick to the ground
    ))
  (Physics|AddForce (Variables|Default|GetBodyPrimitive) (Variables|Default|GetMovementAcceleration) "None" true))

(fn MoveonGround
  (params (TargetDirection :type Vector))
  (bind _desiredvelocityoffset (Variables|Default|GetDesiredVelocityOffset))
  (bind _bodyprimitive (Variables|Default|GetBodyPrimitive))
  (bind _speedmax (Variables|MovementStats|GetSpeedMax))
  (bind _speedmaxmultiplierstatic (Variables|MovementStats|GetSpeedMaxMultiplierStatic))
  (bind _returnvalue (* _speedmax _speedmaxmultiplierstatic))
  (bind _returnvalue_2 (* TargetDirection _returnvalue))
  (bind _returnvalue_3 (+ _desiredvelocityoffset _returnvalue_2))
  (bind _returnvalue_4 (Physics|GetPhysicsLinearVelocity (Variables|Default|GetBodyPrimitive) "None"))
  (bind _output_get (Variables|Default|SetLinearVelocity2D (* _returnvalue_4 "1.000000,1.000000, 0")))
  ;[1 1 1] Update state and local variables
  (Variables|Default|SetCurrentForwardSpeed (Math|Vector|VectorLength _output_get))
  (bind _output_get_2 (Variables|Default|SetDesiredVelocity _returnvalue_3))
  (Variables|Default|SetVelocityDotInput (Math|Vector|DotProduct _returnvalue_3 (Variables|Default|GetLinearVelocity2D)))
  (Physics|AddForce (Variables|Default|GetBodyPrimitive) (* (Variables|Default|GetKnockbackAcceleration) (Variables|Default|GetKnockback%20Effect%20Multiplier)) "None" true :!pinned true) ; Apply knockback
  (Variables|Default|SetKnockbackAcceleration "0, 0, 0")
  ;[0.15 0.15 0.15 0.5] Determine if Braking
  (Variables|Default|SetMovementAcceleration (* (Math|Vector|VectorClampSize2D (- _output_get_2 (Variables|Default|GetLinearVelocity2D)) 0.0 (* (Math|Curves|GetFloatValue (Variables|MovementStats|GetAcceleration%20Curve) (/ (Variables|Default|GetCurrentForwardSpeed) (* (Variables|MovementStats|GetSpeedMax) (Variables|MovementStats|GetSpeedMaxMultiplierCurrent)))) (* (Variables|MovementStats|GetAccelerationMax) (Variables|MovementStats|GetAccelerationMultiplier)))) 1.0))
  (if (and (or (<= (Variables|Default|GetVelocityDotInput) 1e+03) (Math|Vector|VectorIsNearlyZero TargetDirection)) (not (Variables|Default|GetisDashing))) ; Should we be braking?
    ;[0.15 0.15 0.15 0.5] Brake
    (Physics|AddForce _bodyprimitive (* (Variables|Default|GetLinearVelocity2D) (* (Math|Float|MapRangeClamped (Variables|Default|GetVelocityDotInput) 0.0 (Variables|MovementStats|GetSpeedMax) 0.0 (Variables|MovementStats|GetBrakingFriction)) (* (Physics|GetMass _bodyprimitive) -9.8e+02))) "None" false :!pinned true) ; Apply friction force
  )
  (return))

(fn AddKnockback
  (params (Force :type Vector))
  (Variables|Default|SetKnockbackAcceleration (+ (Variables|Default|GetKnockbackAcceleration) Force)))

(fn AddSpeedModifier
  (params (modification :type Float%20%28double-precision%29))
  (bind _returnvalue (Utilities|Array|Add (Variables|MovementStats|GetSpeedMaxMultiplierEffectsDynamic) modification))
  (CallFunction|UpdateSpeedModifier)
  (return _returnvalue))

(fn UpdateSpeedModifier
  (for _array_element (Variables|MovementStats|GetSpeedMaxMultiplierEffectsDynamic) ; Apply all temporary speed modifiers
    (LocalVariables|SetRunningTotal (+ _array_element (LocalVariables|GetRunningTotal))))
  (bind _output_get (Variables|MovementStats|SetSpeedMaxMultiplierCurrent (* (+ (LocalVariables|GetRunningTotal) 1.0) (Variables|MovementStats|GetSpeedMaxMultiplierStatic)))))

(fn RemoveSpeedModifier
  (params (modification%20ID :type Integer))
  (Utilities|Array|RemoveIndex (Variables|MovementStats|GetSpeedMaxMultiplierEffectsDynamic) modification%20ID)
  (CallFunction|UpdateSpeedModifier)
  (return))

(fn ModifySpeedModifier
  (params (modification%20ID :type Integer) (new%20value :type Float%20%28double-precision%29))
  (Utilities|Array|SetArrayElem (Variables|MovementStats|GetSpeedMaxMultiplierEffectsDynamic) modification%20ID new%20value)
  (CallFunction|UpdateSpeedModifier)
  (return))