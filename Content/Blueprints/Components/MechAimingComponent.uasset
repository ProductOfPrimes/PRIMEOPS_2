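; Component that rotates a mech's torso toward the current 2D aim input by updating a replicated torso azimuth.
; Aim measures the azimuth error, accelerates angular velocity toward it, and clamps speed using a curve of that error, a maximum and a multiplier.
; The server applies double the client's acceleration to slightly offset input lag.
; Zero input stops rotation instantly, and the azimuth's OnRep handler is empty.
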(fn Aim
  (bind _currentaiminput (Variables|Default|GetCurrentAimInput))
  (if (Class|KismetMathLibrary|IsNearlyZero2D _currentaiminput 0.0001)
    (Variables|Default|SetAngularVelocity 0.0)
    (else
      (LocalVariables|SetazimuthDifference (.Azimuth (Class|KismetMathLibrary|GetAzimuthandElevation (Math|Conversions|ToVector(Vector2D) _currentaiminput) (Math|Transform|MakeTransform "0, 0, 0" (Math|Vector|RotatorfromAxisandAngle "0, 0,1.000000" (Variables|Default|GetTorsoAzimuth))))))
      (bind _output_get (Variables|Default|SetAngularVelocity (Math|Float|Clamp(Float) (+ (* (Utilities|Time|GetWorldDeltaSeconds) (Variables|Default|GetAimAcceleration) (Math|Float|Sign(Float) (LocalVariables|GetazimuthDifference)) (Math|Float|SelectFloat 2.0 1.0 (Networking|IsServer))) (Variables|Default|GetAngularVelocity)) (* (* (Variables|AimStats|GetTorsoRotationSpeedMax) (Math|Curves|GetFloatValue (Variables|Default|GetazimuthToSpeedfunction) (Math|Float|Absolute(Float) (/ (LocalVariables|GetazimuthDifference) 1.8e+02))) (Variables|AimStats|GetTorsoRotationSpeedMultiplier)) -1.0) (* (Variables|AimStats|GetTorsoRotationSpeedMax) (Math|Curves|GetFloatValue (Variables|Default|GetazimuthToSpeedfunction) (Math|Float|Absolute(Float) (/ (LocalVariables|GetazimuthDifference) 1.8e+02))) (Variables|AimStats|GetTorsoRotationSpeedMultiplier)))))
      ;[1 1 1] Add to azimuth
      (Variables|Default|SetTorsoAzimuth (Math|Float|%(Float) (+ (Variables|Default|GetTorsoAzimuth) (* _output_get (Utilities|Time|GetWorldDeltaSeconds))) 3.6e+02))))
  (return (Variables|Default|GetAngularVelocity)))

(fn OnRepTorsoAzimuth)