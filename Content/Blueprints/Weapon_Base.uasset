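; Weapon_Base is a base weapon Blueprint that handles burst firing and cooldown, with an empty Fire function as the hook for the actual shot.
; Activate queues a burst when the weapon is off cooldown and idle.
; Tick spends the queue at the burst interval, using a while loop to allow several shots per frame, then runs the cooldown and signals EventOnCooldownFinish.
; The construction script defaults to single-shot bursts.
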(event EventBeginPlay)

(event Collision|EventActorBeginOverlap
  (params (OtherActor :type Actor%20Object%20Reference)))

(event EventTick
  (params (DeltaSeconds :type Float%20%28single-precision%29))
  (bind _burstshotbulletstofire (Variables|ProjectileProperties|GetBurstShotBulletsToFire))
  ;[1 1 1] Any burst shot bullets to fire?
  (if (> (Variables|ProjectileProperties|GetBurstShotBulletsToFire) 0)
    (bind _output_get (Variables|ProjectileProperties|SetBurstShotCooldownTimer (- (Variables|ProjectileProperties|GetBurstShotCooldownTimer) DeltaSeconds)))
    (while (< _output_get 0.0)
      (Variables|ProjectileProperties|SetBurstShotCooldownTimer (+ _output_get (Variables|ProjectileProperties|GetBurstShotCooldown)))
      (Math|Integer|DecrementInt _burstshotbulletstofire
        (:%20%20
          (CallFunction|Fire) ; Around here is where we add heat and haptic feedback
          (if (== _burstshotbulletstofire 0)
            (Variables|Default|SetCooldownTimer (Variables|Default|GetCooldownTime))
            (Variables|ProjectileProperties|SetBurstShotCooldownTimer (Variables|ProjectileProperties|GetBurstShotCooldown))))))
    (else
      (bind _output_get_2 (Variables|Default|SetCooldownTimer (- (Variables|Default|GetCooldownTimer) DeltaSeconds)))
      (if (and (Variables|Default|GetOnCooldown) (< (- (Variables|Default|GetCooldownTimer) DeltaSeconds) 0.0))
        ;[1 1 1] Invoke OnCooldownFinish when cooldown timer goes below 0
        (Variables|Default|SetCooldownTimer 0.0)
        (Variables|Default|SetOnCooldown false)
        (CallFunction|EventonCooldownFinish)
        (elif (> _output_get_2 0.0)
          (Variables|Default|SetOnCooldown true))))))

(fn ConstructionScript
  (Variables|Default|SetCooldownTimer 0.0)
  (Variables|ProjectileProperties|SetBurstCount 1)
  (Variables|ProjectileProperties|SetBurstShotCooldown 0.0)
  (Variables|ProjectileProperties|SetBurstShotBulletsToFire 0)
  (Variables|ProjectileProperties|SetBurstShotCooldownTimer 0.0))

(fn Fire)

(fn Activate
  (if (and (not (Variables|Default|GetOnCooldown)) (== (Variables|ProjectileProperties|GetBurstShotBulletsToFire) 0))
    (Variables|ProjectileProperties|SetBurstShotBulletsToFire (Variables|ProjectileProperties|GetBurstCount))))