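; Mech radiator that tracks heat and signals overheat warning, overheat and recovery through event dispatchers.
; AddHeat raises temperature and pauses cooling on positive amounts; Tick resumes it after a delay, with CoolOff lowering heat and checking recovery thresholds.
; Its own dispatcher handlers set state, play sounds and start or stop looping controller rumble.
; Rumble intensity follows temperature or overheat state, while attached Niagara steam receives the heat percentage during cooling.
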(event Custom|CustomEvent)

(event Custom|OnOverheatRecover
  (bind _rumble (Variables|Default|GetRumble))
  (Variables|Default|SetOverheated false)
  (Audio|PlaySound2D "/Game/Audio/Sound/Menu_Back.Menu_Back" 1.0 1.0 0.0 0 0)
  (Audio|Components|Audio|Stop _rumble)
  (Class|ForceFeedbackComponent|SetIntensityMultiplier _rumble 0.0))

(event Custom|OverheatWarningRecovered
  (bind _rumble (Variables|Default|GetRumble))
  (Variables|Default|SetOverheatWarningIssued false)
  (Audio|Components|Audio|Stop _rumble)
  (Class|ForceFeedbackComponent|SetIntensityMultiplier _rumble 0.0))

(event Custom|OverheatWarning
  (Variables|Default|SetOverheatWarningIssued true)
  (Audio|PlaySound2D "/Game/Audio/Sound/OverheatWarning.OverheatWarning" 1.0 1.0 0.0 0 0)
  (Audio|Components|Audio|Play (Variables|Default|GetRumble) 0.0))

(event Custom|OnOverheat
  (Variables|Default|SetOverheated true)
  (Audio|PlaySound2D "/Game/Audio/Sound/Overheat.Overheat" 1.0 1.0 0.0 0 0))

(event EventBeginPlay
  (bind _returnvalue (Niagara|SpawnSystemAttached "/Game/VFX/NS_heatSteam.NS_heatSteam" self "None" "0, 0, 0" "0, 0, 0" "KeepRelativeOffset" false))
  (Variables|Default|SetHeatSteam _returnvalue)
  (bind _returnvalue_2 (ForceFeedback|SpawnForceFeedbackAttached "/Game/HeatRumble.HeatRumble" self "None" "0, 0, 0" "0, 0, 0" "SnapToTarget" true true 1.0 0.0 0 false))
  (Variables|Default|SetRumble _returnvalue_2)
  (EventDispatchers|BindEventtoDispatcheronOverheat (delegate Custom|OnOverheat))
  (EventDispatchers|BindEventtoDispatcheronOverheatRecover (delegate Custom|OnOverheatRecover))
  (EventDispatchers|BindEventtoDispatcheronOverheatWarning (delegate Custom|OverheatWarning))
  (EventDispatchers|BindEventtoDispatcheronOverheatWarningRecover (delegate Custom|OverheatWarningRecovered)))

(event EventTick
  (params (DeltaSeconds :type Float%20%28single-precision%29))
  (bind _rumble (Variables|Default|GetRumble))
  ;[1 1 1] Heat Haptic Feedback
  (if (Variables|Default|GetOverheated)
    (Class|ForceFeedbackComponent|SetIntensityMultiplier _rumble 0.9)
    (else
      (bind _temppercent (CallFunction|GetTempPercent))
      (Class|ForceFeedbackComponent|SetIntensityMultiplier _rumble (Math|Float|MapRangeClamped _temppercent (Variables|Default|GetOverheatWarningThresholdPercentage) 1.0 0.0 0.15))))
  (if (Variables|Default|GetisCooling)
    (CallFunction|CoolOff DeltaSeconds)
    (else
      (Utilities|FlowControl|Delay (Variables|Default|GetCoolDelay))
      (Variables|Default|SetisCooling true))))

(fn AddHeat
  (params (Amount :type Float%20%28single-precision%29))
  (Variables|Default|SetCurrentTemp (Math|Float|Max(Float) (+ (Variables|Default|GetCurrentTemp) Amount) 0.0))
  (Variables|Default|SetisCooling (<= Amount 0.0))
  (if (and (> (Variables|Default|GetCurrentTemp) (Variables|Default|GetMaxTemp)) (not (Variables|Default|GetOverheated)))
    (Default|CallDispatcheronOverheat)
    (return)
    (elif (and (> (Variables|Default|GetCurrentTemp) (* (Variables|Default|GetOverheatWarningThresholdPercentage) (Variables|Default|GetMaxTemp))) (not (Variables|Default|GetOverheatWarningIssued)))
      (Default|CallDispatcheronOverheatWarning)
      (return)
      (else
        (return)))))

(fn GetTempPercent
  (return (/ (Variables|Default|GetCurrentTemp) (Variables|Default|GetMaxTemp))))

(fn CoolOff
  (params (dt :type Float%20%28single-precision%29))
  (Variables|Default|SetCurrentTemp (Math|Float|Clamp(Float) (- (Variables|Default|GetCurrentTemp) (* dt (Variables|Default|GetCoolRate))) 0.0 3e+05))
  (bind _temppercent (CallFunction|GetTempPercent))
  (Effects|Components|ParticleSystem|SetFloatParameter (Variables|Default|GetHeatSteam) "HeatPercentage" _temppercent) ; Update particle system parameter
  (if (Variables|Default|GetOverheated)
    (if (<= _temppercent (Variables|Default|GetOverheatCooldownThresholdPercentage))
      (Default|CallDispatcheronOverheatRecover))
    (elif (and (<= _temppercent (Variables|Default|GetOverheatWarningThresholdPercentage)) (Variables|Default|GetOverheatWarningIssued))
      (Default|CallDispatcheronOverheatWarningRecover))))