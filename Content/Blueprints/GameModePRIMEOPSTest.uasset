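; Game mode for local multiplayer mech battles, won by the last team standing.
; On BeginPlay it creates local players from MadMechsGameInstance slots, spawns team-assigned mechs with chosen loadouts, and points player 0's view at the level's CameraController.
; Each death event updates the TeamEliminationStatus map, checks for a winner and refreshes the camera's mech array.
; A win plays the team's music, shows colored victory text on the GetReady widget, then opens MainMenu.
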(event Custom|FindCamera
  (bind _outactors (Actor|GetAllActorsOfClass "/Game/Blueprints/CameraController.CameraController_C"))
  (bind _output_get (Variables|Default|SetCam (Utilities|Array|Get(acopy) _outactors)))
  (Default|InitializeMechArray _output_get))

(event Custom|EventDispatcherDeath_Event
  (params (Team :type Team%20Enum :default "NewEnumerator0") (Player%20Number :type Integer) (Instigator :type Actor%20Object%20Reference))
  (Utilities|FlowControl|Sequence
    (:then_0
      (Development|PrintString (Utilities|String|BuildString(Integer) (Utilities|String|BuildString(Name) "Gamemode says... " "" (Utilities|String|StringToName (Utilities|GetDisplayName Instigator)) " killed ") "player " Player%20Number (Utilities|String|Append " on team " (Utilities|String|EnumtoString Team))) true true "(R=0.980592,G=0.000000,B=1.000000,A=1.000000)" 1e+01)
      (bind _isteamdead (CallFunction|UpdateLossConditionElimination Team))
      (if _isteamdead
        (Development|PrintString (Utilities|String|Append (Utilities|String|EnumtoString Team) " ELIMINATED! ////////////////////") true true "(R=1.000000,G=0.000000,B=0.835386,A=1.000000)" 1e+01)
        ;[1 1 1] Check Every Other Team, to see if they won
        (bind _keys (Utilities|Map|Keys (Variables|Default|GetTeamEliminationStatus)))
        (for _array_element _keys
          (if (!= _array_element Team)
            (bind _victory (CallFunction|VictoryConditionElimination (Utilities|Enum|ByteToEnumTeam _array_element)))
            (if _victory
              (Development|PrintString (Utilities|String|Append (Utilities|String|EnumtoString (Utilities|Enum|ByteToEnumTeam _array_element)) " TEAM WINS ") true true "(R=1.000000,G=0.000000,B=0.835386,A=1.000000)" 1e+01)
              (Audio|PlaySound2D (Utilities|Select :Index (Utilities|Enum|ByteToEnumTeam _array_element) :NewEnumerator0 "/Game/Audio/Music/BlacificBeat.BlacificBeat" :NewEnumerator1 "/Game/Audio/Music/BlacificBlenu_Converted.BlacificBlenu_Converted" :NewEnumerator5 0 :NewEnumerator6 0 :NewEnumerator7 0 :NewEnumerator8 0 :NewEnumerator2 "/Game/Audio/Music/BlacificBlim.BlacificBlim" :NewEnumerator4 0 :NewEnumerator3 0) 1.0 0.5 0.0 0 0) ; AMPED UP AND BASS BOOSTED FOR YOUR LISTENING PLEASURE
              (bind _asgame_hud (Utilities|Casting|CastToGameHUD (HUD|GetHUD (Game|GetPlayerController 0))))
              (Widget|SetVisibility (UserInterface|GetUserWidgetObject (Variables|/Game/UI/Gameplay/GameHUD.GameHUD_C|GetReady _asgame_hud)) "Visible")
              (bind _asget_ready_ui (Utilities|Casting|CastToGetReadyUI (UserInterface|GetUserWidgetObject (Variables|/Game/UI/Gameplay/GameHUD.GameHUD_C|GetReady _asgame_hud))))
              (Rendering|Components|TextRender|SetText (Variables|/Game/UI/Gameplay/GetReadyUI.GetReadyUI_C|GetRichTextBlock_70 _asget_ready_ui) (Utilities|Text|ToText(String) (Utilities|String|Append (Utilities|String|EnumtoString (Utilities|Enum|ByteToEnumTeam _array_element)) " TEAM WINS ")))
              (Class|RichTextBlock|SetDefaultColorandOpacity (Variables|/Game/UI/Gameplay/GetReadyUI.GetReadyUI_C|GetRichTextBlock_70 _asget_ready_ui) (Utilities|Select :Index (Utilities|Enum|ByteToEnumTeam _array_element) :NewEnumerator0 (Utilities|Struct|MakeSlateColor "(R=0.838542,G=0.000000,B=0.000000,A=1.000000)") :NewEnumerator1 (Utilities|Struct|MakeSlateColor "(R=0.000000,G=0.141000,B=0.807292,A=1.000000)") :NewEnumerator5 "" :NewEnumerator6 "" :NewEnumerator7 "" :NewEnumerator8 "" :NewEnumerator2 (Utilities|Struct|MakeSlateColor "(R=0.312500,G=0.312500,B=0.312500,A=1.000000)") :NewEnumerator4 "" :NewEnumerator3 ""))
              (Utilities|FlowControl|Delay 5.0)
              (Game|OpenLevel(byName) "MainMenu"))))))
    (:then_2
      (Default|InitializeMechArray (Variables|Default|GetCam)))))

(event EventBeginPlay
  (Audio|PlaySound2D "/Game/Audio/Sound/Battle_Ready.Battle_Ready" 1.0 1.0 0.0 0 0)
  (CallFunction|SpawnPlayers)
  (CallFunction|FindCamera)
  (Game|Player|SetViewTargetwithBlend (Game|GetPlayerController 0) (Variables|Default|GetCam) 0.0 "VTBlend_Linear" 0.0 false)
  (EventDispatchers|BindEventtoEventDispatcherDeath (delegate Custom|EventDispatcherDeath_Event)))

(event EventTick
  (params (DeltaSeconds :type Float%20%28single-precision%29)))

(fn ConstructionScript)

(fn SpawnPlayers
  (bind _asmad_mechs_game_instance (Utilities|Casting|CastToMadMechsGameInstance (Game|GetGameInstance)))
  (LocalVariables|SetMadMechsInstance _asmad_mechs_game_instance)
  (Variables|Default|SetNumPlayers-1 (- (Variables|/Game/Blueprints/MainMenu/MadMechsGameInstance.MadMechsGameInstance_C|GetNumPlayers _asmad_mechs_game_instance) 1))
  (for _index (range 1 (- (Utilities|Array|Length (Variables|/Game/Blueprints/MainMenu/MadMechsGameInstance.MadMechsGameInstance_C|GetPlayerIDToSlot _asmad_mechs_game_instance)) 1))
    (if (!= -1 (Utilities|Array|Get(acopy) (Variables|/Game/Blueprints/MainMenu/MadMechsGameInstance.MadMechsGameInstance_C|GetPlayerIDToSlot _asmad_mechs_game_instance) _index))
      (Class|GameplayStatics|CreatePlayer _index)))
  (for _index_2 (range 0 (- (Utilities|Array|Length (Variables|/Game/Blueprints/MainMenu/MadMechsGameInstance.MadMechsGameInstance_C|GetPlayerIDToSlot _asmad_mechs_game_instance)) 1))
    (if (!= (Utilities|Array|Get(acopy) (Variables|/Game/Blueprints/MainMenu/MadMechsGameInstance.MadMechsGameInstance_C|GetPlayerIDToSlot _asmad_mechs_game_instance) _index_2) -1)
      (bind _returnvalue (Game|SpawnActorfromClass "/Game/Blueprints/Mech_Pawn.Mech_Pawn_C" (Math|Transform|MakeTransform "0, 0,1000.000000") "AdjustIfPossibleButAlwaysSpawn" "OverrideRootScale" 0 _index_2 (Utilities|Array|Get(acopy) (Variables|/Game/Blueprints/MainMenu/MadMechsGameInstance.MadMechsGameInstance_C|GetTeams (LocalVariables|GetMadMechsInstance)) _index_2) 0))
      (Utilities|Array|Add (Variables|Default|GetMechs) _returnvalue)
      (Utilities|Map|Add (Variables|Default|GetTeamEliminationStatus) (Utilities|Array|Get(acopy) (Variables|/Game/Blueprints/MainMenu/MadMechsGameInstance.MadMechsGameInstance_C|GetTeams (LocalVariables|GetMadMechsInstance)) _index_2) (Class|KismetSystemLibrary|MakeLiteralBool false))
      (Pawn|Possess (Game|GetPlayerController _index_2) _returnvalue)
      ;[1 1 1] Apply Loadout
      (Default|DefineStartingLoadout (Variables|/Game/Blueprints/Mech_Pawn.Mech_Pawn_C|GetMechWeaponHandlerBP _returnvalue) (Utilities|Struct|BreakPlayerLoadout (Utilities|Array|Get(acopy) (Variables|/Game/Blueprints/MainMenu/MadMechsGameInstance.MadMechsGameInstance_C|GetLoadouts (LocalVariables|GetMadMechsInstance)) (Variables|/Game/Blueprints/Mech_Pawn.Mech_Pawn_C|GetPlayerInt _returnvalue)))))))

(fn UpdateLossConditionElimination
  (params (Team :type Team%20Enum :default "NewEnumerator2"))
  (bind _numalive (LocalVariables|GetNumAlive))
  (bind _returnvalue (== _numalive 0))
  (bind _array_element (Utilities|Array|ForEachLoopwithBreak (Variables|Default|GetMechs) :!label _label)
    (:LoopBody
      (if (== (Variables|/Game/Blueprints/Mech_Pawn.Mech_Pawn_C|GetTeam _array_element) Team)
        (if (Variables|/Game/Blueprints/LivingActorComponent.LivingActorComponent_C|GetisAlive (Variables|/Game/Blueprints/Mech_Pawn.Mech_Pawn_C|GetLivingActorComponent _array_element))
          (Math|Integer|IncrementInt (LocalVariables|GetNumAlive)
            (:%20%20
              (goto _label Break))))))
    (:Completed
      (Utilities|Map|Add (Variables|Default|GetTeamEliminationStatus) Team _returnvalue)
      (return _returnvalue))))

(fn ChooseRandomTeam
  (switch int (Math|Random|RandomIntegerinRange 0 2)
    (:0
      (return "NewEnumerator0"))
    (:1
      (return "NewEnumerator1"))
    (:2
      (return "NewEnumerator2"))))

(fn VictoryConditionElimination
  (params (Team :type Team%20Enum :default "NewEnumerator0"))
  ;[1 1 1] Check if all teams except mine...
  (bind _keys (Utilities|Map|Keys (Variables|Default|GetTeamEliminationStatus)))
  (for _array_element _keys
    (if (!= _array_element Team)
      ;[1 1 1] Is the team dead? If not, return/break. No chicken dinner today
      (if (not (.Value (Utilities|Map|Find (Variables|Default|GetTeamEliminationStatus) _array_element)))
        (return false))))
  (return true))