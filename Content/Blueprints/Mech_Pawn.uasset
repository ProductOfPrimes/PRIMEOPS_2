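; Player mech pawn for team-based local multiplayer, assembled from leader-posed body parts and spawned above its tagged PlayerStart.
; Profile-mapped controller or mouse input drives movement and aiming components and four weapon-handler gear slots.
; Radiator heat and health feed the player UI, with team-damage filtering on hits.
; Non-environmental kills start a doomed countdown that slows the mech and ramps heat before a radial-damage explosion; environmental kills die immediately.
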(event Custom|LeftArmEvent
  (params (Pressed? :type Boolean))
  (bind _output_get (Variables|Inputs|SetLeftHandPressed Pressed?))
  (if (not _output_get)
    ;[1 1 1] Gear DeActivation
    (Default|DeActivateSlot (Variables|Components|GetMechWeaponHandlerBP) (Utilities|Enum|LiteralenumGearSlot "L_ARM"))))

(event Custom|LeftShoulderEvent
  (params (Pressed? :type Boolean))
  (bind _output_get (Variables|Inputs|SetLeftShoulderPressed Pressed?))
  (if (not _output_get)
    ;[1 1 1] Gear DeActivation
    (Default|DeActivateSlot (Variables|Components|GetMechWeaponHandlerBP) (Utilities|Enum|LiteralenumGearSlot "L_SHD"))))

(event Custom|RightShoulderEvent
  (params (Pressed? :type Boolean))
  (bind _output_get (Variables|Inputs|SetRightShoulderPressed Pressed?))
  (if (not _output_get)
    ;[1 1 1] Gear DeActivation
    (Default|DeActivateSlot (Variables|Components|GetMechWeaponHandlerBP) (Utilities|Enum|LiteralenumGearSlot "R_SHD"))))

(event Custom|RightArmEvent
  (params (Pressed? :type Boolean))
  (bind _output_get (Variables|Inputs|SetRightHandPressed Pressed?))
  (if (not _output_get)
    ;[1 1 1] Gear DeActivation
    (Default|DeActivateSlot (Variables|Components|GetMechWeaponHandlerBP) (Utilities|Enum|LiteralenumGearSlot "R_ARM"))))

(event EventBeginPlay
  (Utilities|FlowControl|Sequence
    (:then_0
      (CallFunction|Spawn)
      (Variables|/Game/Blueprints/Abilities/MechWeaponHandlerBP.MechWeaponHandlerBP_C|SetMech%20Owner (Variables|Components|GetMechWeaponHandlerBP) self))
    (:then_1
      (Variables|/Script/Engine.SkeletalMeshComponent|SetbPauseAnims (Variables|Components|Getlegs_01) true)
      (Utilities|FlowControl|Delay (/ (Math|Conversions|ToFloat(Integer) (Variables|Default|GetPlayerInt)) 2.0))
      (Variables|/Script/Engine.SkeletalMeshComponent|SetbPauseAnims (Variables|Components|Getlegs_01) false))
    (:then_2
      (bind _asmain_player_ui (Utilities|Casting|CastToMainPlayerUI (UserInterface|GetUserWidgetObject (Variables|Components|GetHUD))))
      (Default|UpdatePlayerIndicator _asmain_player_ui (Utilities|Text|FormatText "P{PlayerNum}" (+ (Variables|Default|GetPlayerInt) 1)) (Variables|Default|GetTeam))
      (bind _temppercent (Default|GetTempPercent (Variables|Components|GetMechRadiator)))
      (CallFunction|UpdateTempUI _temppercent)
      (Utilities|FlowControl|Delay (Variables|InitVars|GetInitDelay))
      (Variables|InitVars|SetCanAct true))
    (:then_3
      (Variables|/Game/Blueprints/ControlMapping/ProfileMapComponent.ProfileMapComponent_C|SetController (Variables|Default|GetProfileMapComponent) (Game|GetPlayerController (Variables|Default|GetPlayerInt)))
      (Utilities|FlowControl|Sequence
        (:then_0
          (EventDispatchers|BindEventtoLeftArmEvent (Variables|Default|GetProfileMapComponent) (delegate Custom|LeftArmEvent)))
        (:then_1
          (EventDispatchers|BindEventtoLeftShoulderEvent (Variables|Default|GetProfileMapComponent) (delegate Custom|LeftShoulderEvent)))
        (:then_2
          (EventDispatchers|BindEventtoRightShoulderEvent (Variables|Default|GetProfileMapComponent) (delegate Custom|RightShoulderEvent)))
        (:then_3
          (EventDispatchers|BindEventtoRightArmEvent (Variables|Default|GetProfileMapComponent) (delegate Custom|RightArmEvent)))))))

(event EventDestroyed
  ;[1 1 1] Destroy
  (bind _returnvalue (Actor|GetActorOfClass "/Game/Blueprints/CameraController.CameraController_C"))
  (Game|Player|SetViewTargetwithBlend (Game|GetPlayerController (Variables|Default|GetPlayerInt)) _returnvalue 0.0 "VTBlend_Linear" 0.0 false))

(event EventTick
  (params (DeltaSeconds :type Float%20%28single-precision%29))
  (bind _playerint (Variables|Default|GetPlayerInt))
  (bind _returnvalue (Game|GetPlayerController _playerint))
  (bind (_locationx _locationy) (Game|Player|GetMousePosition _returnvalue))
  (if (Variables|InitVars|GetCanAct)
    (Utilities|FlowControl|Sequence
      (:then_0
        (if (.iscontroller (Variables|/Game/Blueprints/ControlMapping/ProfileMapComponent.ProfileMapComponent_C|GetProfile (Variables|Default|GetProfileMapComponent)))
          (Variables|Inputs|SetMoveInput (Math|Vector|MakeVector (Class|Actor|GetInputAxisKeyValue) (Class|Actor|GetInputAxisKeyValue) 0.0))
          (Variables|Inputs|SetAimInput (Math|Vector|MakeVector (Class|Actor|GetInputAxisKeyValue) (Class|Actor|GetInputAxisKeyValue) 0.0))
          (else
            (bind _newparam2 (Utilities|ScreenPointNormalized (Math|Vector2D|MakeVector2D _locationx _locationy))
              (:NewParam3
                (bind _newparam2_2 (Utilities|ScreenPointNormalized (.ScreenPosition (Class|GameplayStatics|ProjectWorldtoScreen (Game|GetPlayerController (Variables|Default|GetPlayerInt)) (Transformation|GetActorLocation) false)))
                  (:NewParam3
                    (Variables|Inputs|SetMoveInput (Math|Vector|MakeVector (Input|AxisValues|GetMoveForward) (Input|AxisValues|GetMoveRight) 0.0))
                    (Variables|Inputs|SetAimInput (Math|Vector|Normalize (Math|Vector|MakeVector (.x (- _newparam2 _newparam2_2)) (.y (- _newparam2 _newparam2_2)) 0.0))))))))))
      (:then_1
        (Default|MoveonGround (Variables|Components|GetMechMovementComponent) (Variables|Inputs|GetMoveInput))
        (bind _turnspeed (Default|Aim (Variables|Components|GetMechAimingComponent) (Variables|Inputs|GetAimInput)))
        (Utilities|PlayTurningSound _turnspeed))
      (:then_2
        ;[1 1 1] Temperature
        (bind _temppercent (Default|GetTempPercent (Variables|Components|GetMechRadiator)))
        (CallFunction|UpdateTempUI _temppercent)
        (Rendering|Material|SetScalarParameterValue (Variables|Default|GetradiatorMat) "ParamHeat" _temppercent :!class /Script/Engine.MaterialInstanceDynamic))
      (:then_3
        ;[1 1 1] Gear Activation
        (Utilities|FlowControl|Sequence
          (:then_0
            (if (Variables|Inputs|GetLeftHandPressed)
              (Default|ActivateSlot (Variables|Components|GetMechWeaponHandlerBP) (Utilities|Enum|LiteralenumGearSlot "L_ARM"))))
          (:then_1
            (if (Variables|Inputs|GetLeftShoulderPressed)
              (Default|ActivateSlot (Variables|Components|GetMechWeaponHandlerBP) (Utilities|Enum|LiteralenumGearSlot "L_SHD"))))
          (:then_2
            (if (Variables|Inputs|GetRightShoulderPressed)
              (Default|ActivateSlot (Variables|Components|GetMechWeaponHandlerBP) (Utilities|Enum|LiteralenumGearSlot "R_SHD"))))
          (:then_3
            (if (Variables|Inputs|GetRightHandPressed)
              (Default|ActivateSlot (Variables|Components|GetMechWeaponHandlerBP) (Utilities|Enum|LiteralenumGearSlot "R_ARM"))))))
      (:then_4
        (if (Variables|Death|GetIsDoomed)
          (Utilities|TickDoomedState))))))

(event Game|Damage|EventAnyDamage
  (params (Damage :type Float%20%28single-precision%29) (DamageType :type Damage%20Type%20Object%20Reference) (InstigatedBy :type Controller%20Object%20Reference) (DamageCauser :type Actor%20Object%20Reference))
  (Utilities|IsValid InstigatedBy
    (:Is%20Valid
      (if (Variables|Default|GetTeamDamageEnabled)
        (bind _killingblow (Default|TakeDamage (Variables|Components|GetLivingActorComponent) Damage :!label _label))
        (Utilities|FlowControl|Sequence
          (:then_0
            (CallFunction|UpdateHealthUI))
          (:then_1
            (if _killingblow ; Was this a kill?
              (if (!= (Utilities|GetClass DamageType) "/Engine/EngineDamageTypes/DmgTypeBP_Environmental.DmgTypeBP_Environmental_C") ; Should enter doomed state?
                ;[1 1 1] Death
                (CallFunction|EnterDoomedState)
                (else
                  (Default|CallOnDeath)
                  (CallFunction|Die)
                  (Development|PrintString (Utilities|String|Append (Utilities|GetDisplayName self) "Died to environmental damage"))
                  (Utilities|FlowControl|Delay 1.0)
                  (Actor|DestroyActor))))))
        (else
          (bind _asmech_pawn (Utilities|Casting|CastToMech_Pawn (Pawn|GetControlledPawn InstigatedBy))
            (:then
              (if (!= (Variables|Mech_Pawn_C|GetTeam _asmech_pawn) (Variables|Default|GetTeam))
                (goto _label)))
            (:CastFailed
              (goto _label))))))
    (:Is%20Not%20Valid
      (goto _label))))

(event EventEndPlay
  (params (EndPlayReason :type EEndPlayReason%20Enum :default "Destroyed"))
  ;[1 1 1] End Play
)

(event Input|KeyboardEvents|D
  (params (Key :type Key%20Structure :default "None"))
  (:Pressed
    (Game|Damage|ApplyDamage self 1e+02 0 0 "/Script/Engine.DamageType")))

(event Input|KeyboardEvents|H
  (params (Key :type Key%20Structure :default "None"))
  (:Pressed
    (CallFunction|AddHeat -1e+01)))

(fn ConstructionScript
  (Components|SkinnedMesh|SetLeaderPoseComponent (Variables|Components|Gethead_01) (Variables|Components|Getlegs_01) false false)
  (Variables|/Game/Blueprints/LivingActorComponent.LivingActorComponent_C|SetTeam (Variables|Components|GetLivingActorComponent) (Variables|Default|GetTeam))
  (Variables|/Game/Blueprints/Components/MechMovementComponent.MechMovementComponent_C|SetBodyPrimitive (Variables|Components|GetMechMovementComponent) (Variables|Components|GetTerrainCollision))
  (Transformation|AttachComponentToComponent (Variables|Components|GetMechRadiator) (Variables|Components|Getlegs_01) "RadiatorSocket" "SnapToTarget" "SnapToTarget" "KeepRelative" false)
  (bind _dynamic_materials (CallFunction|MakeMaterialsDynamic (Variables|Components|GetMechRadiator)))
  (Variables|Default|SetradiatorMat (Utilities|Array|Get(acopy) _dynamic_materials (Utilities|Array|LastIndex _dynamic_materials))))

(fn AddHeat
  (params (Amount :type Float%20%28double-precision%29))
  (bind _mechradiator (Variables|Components|GetMechRadiator))
  (Default|AddHeat (Variables|Components|GetMechRadiator) Amount)
  (bind _asmain_player_ui (Utilities|Casting|CastToMainPlayerUI (UserInterface|GetUserWidgetObject (Variables|Components|GetHUD))))
  (Default|CallAddHeat _asmain_player_ui (Math|Float|SelectFloat (* (Variables|/Game/Blueprints/MechRadiator.MechRadiator_C|GetCoolDelay _mechradiator) 1.0) 0.0 (Variables|/Game/Blueprints/MechRadiator.MechRadiator_C|GetisCooling _mechradiator))))

(fn UpdateTempUI
  (params (TempPercent :type Float%20%28double-precision%29))
  (bind _mechradiator (Variables|Components|GetMechRadiator))
  (bind _asmain_player_ui (Utilities|Casting|CastToMainPlayerUI (UserInterface|GetUserWidgetObject (Variables|Components|GetHUD))))
  (Default|UpdateTemp _asmain_player_ui TempPercent (Variables|/Game/Blueprints/MechRadiator.MechRadiator_C|GetOverheated _mechradiator) (Variables|/Game/Blueprints/MechRadiator.MechRadiator_C|GetOverheatWarningIssued _mechradiator)))

(fn Spawn
  (bind _outactors (Actor|GetAllActorsOfClass "/Script/Engine.PlayerStart"))
  (for _array_element _outactors
    (if (Utilities|Name|Equal(Name) (Variables|/Script/Engine.PlayerStart|GetPlayerStartTag _array_element) (Utilities|String|StringToName (Utilities|String|Append "Player" (Utilities|String|ToString(Integer) (Variables|Default|GetPlayerInt)))))
      (Variables|Default|SetSpawnLocation (Transformation|GetActorTransform _array_element))
      (Transformation|Teleport (+ (Transformation|GetActorLocation _array_element) "0, 0,1000.000000") "0, 0, 0")
      (CallFunction|UpdateMaterialParamstoTeamColor (Utilities|Array|MakeArray (Variables|Components|Getlegs_01) (Variables|Components|Gettorso_01) (Variables|Components|Getshoulder_01_l) (Variables|Components|Getarm_01_l) (Variables|Components|Getarm_01_r) (Variables|Components|Gethead_01) (Variables|Components|Getshoulder_01_r)) (Variables|Default|GetTeam)))))

(fn UpdateHealthUI
  (bind _livingactorcomponent (Variables|Components|GetLivingActorComponent))
  ;[1 1 1] Update HP UI
  (bind _asmain_player_ui (Utilities|Casting|CastToMainPlayerUI (UserInterface|GetUserWidgetObject (Variables|Components|GetHUD))))
  (bind _healthpercent (Default|GetHealthPercent _livingactorcomponent))
  (Default|UpdateHealth _asmain_player_ui _healthpercent (Variables|/Game/Blueprints/LivingActorComponent.LivingActorComponent_C|GetCurrentHealth _livingactorcomponent)))

(fn Die
  (bind _asgame_mode_primeopstest (Utilities|Casting|CastToGameModePRIMEOPSTest (Game|GetGameMode)))
  (Default|EventDispatcherDeathEvent _asgame_mode_primeopstest (Variables|/Game/Blueprints/LivingActorComponent.LivingActorComponent_C|GetTeam (Variables|Components|GetLivingActorComponent)) (Variables|Default|GetPlayerInt))
  (Components|Tick|SetComponentTickEnabled (Variables|Components|Getlegs_01) false)
  (Rendering|Material|SetMaterial (Variables|Components|Getlegs_01) 0 (LocalVariables|GetDeadMaterial))
  (for _array_element (Variables|/Game/Blueprints/Abilities/MechWeaponHandlerBP.MechWeaponHandlerBP_C|GetLoadout (Variables|Components|GetMechWeaponHandlerBP))
    _)
  (Default|SelfDestruct (Variables|Components|GetMechWeaponHandlerBP))
  (Utilities|StopHUDs))

(fn EnterDoomedState
  (Variables|Death|SetDoomedTimer (Variables|Death|GetDoomedTime))
  (Variables|Death|SetIsDoomed true)
  (Audio|PlaySound2D (Variables|Death|GetDeathSirenSound) 0.5 1.0 0.0 0 0)
  (Niagara|SpawnSystemAttached "/Game/VFX/NS_MechCriticalLoop.NS_MechCriticalLoop" (Variables|Components|Getlegs_01) "ChestSocket" "0, 0, 0" "0, 0, 0" "SnapToTarget" false))