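; Component that maps four keys from a control Profile (left and right arm, left and right shoulder) to matching input events.
; Each Tick it polls the Controller for those keys through CheckPressed, then CheckReleased, rather than using input bindings.
; DoOnce gates in each function turn held state into one-shot press and release edges, and each event call passes the key's current down state.
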(event EventBeginPlay)

(event EventTick
  (params (DeltaSeconds :type Float%20%28single-precision%29))
  (Utilities|FlowControl|Sequence
    (:then_0
      (Utilities|CheckPressed))
    (:then_1
      (Utilities|CheckReleased))))