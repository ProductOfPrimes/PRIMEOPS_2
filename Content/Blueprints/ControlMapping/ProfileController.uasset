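; Actor that manages named control-mapping user profiles and persists them through a UserProfilesSaveGame slot.
; On BeginPlay it copies any saved profiles into its UserProfiles map.
; Creating rejects duplicate names, and clearing resets the map to the default controller and keyboard profiles.
; Deleting a default shows a SimpleDialogue warning instead, while every successful change rewrites the slot with a fresh save object.
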(event EventBeginPlay
  (bind _returnvalue (SaveGame|LoadGamefromSlot (Variables|SaveGameIDVars|GetSaveSlotName) (Variables|SaveGameIDVars|GetUserIndex)))
  (bind _asuser_profiles_save_game (Utilities|Casting|CastToUserProfilesSaveGame _returnvalue))
  (bind _output_get (Variables|Default|SetSaveGameInstance _asuser_profiles_save_game))
  (bind _keys (Utilities|Map|Keys (Variables|/Game/Blueprints/ControlMapping/UserProfilesSaveGame.UserProfilesSaveGame_C|GetUserProfiles _output_get)))
  (for _array_element _keys
    (Utilities|Map|Add (Variables|Default|GetUserProfiles) _array_element (.Value (Utilities|Map|Find (Variables|/Game/Blueprints/ControlMapping/UserProfilesSaveGame.UserProfilesSaveGame_C|GetUserProfiles _output_get) _array_element)))))

(event Collision|EventActorBeginOverlap
  (params (OtherActor :type Actor%20Object%20Reference)))

(event EventTick
  (params (DeltaSeconds :type Float%20%28single-precision%29)))

(fn ConstructionScript)

(fn SaveUserProfiles
  (bind _returnvalue (SaveGame|CreateSaveGameObject "/Game/Blueprints/ControlMapping/UserProfilesSaveGame.UserProfilesSaveGame_C"))
  (bind _output_get (Variables|Default|SetSaveGameInstance _returnvalue))
  (Variables|/Game/Blueprints/ControlMapping/UserProfilesSaveGame.UserProfilesSaveGame_C|SetUserProfiles _output_get (Variables|Default|GetUserProfiles))
  (SaveGame|SaveGametoSlot _output_get (Variables|SaveGameIDVars|GetSaveSlotName) (Variables|SaveGameIDVars|GetUserIndex)))

(fn CreateUserProfile
  (params (NewProfileName :type String) (NewProfileContent :type Profile%20Struct%20Structure))
  (bind _userprofiles (Variables|Default|GetUserProfiles))
  (if (Utilities|Map|Contains _userprofiles NewProfileName)
    (return false)
    (else
      (Utilities|Map|Add _userprofiles NewProfileName NewProfileContent)
      (CallFunction|SaveUserProfiles)
      (return true))))

(fn ClearProfiles
  (bind _userprofiles (Variables|Default|GetUserProfiles))
  (Utilities|Map|Clear _userprofiles)
  (Utilities|Map|Add _userprofiles (.profilename (Variables|Defaults|GetDefaultController)) (Variables|Defaults|GetDefaultController))
  (Utilities|Map|Add _userprofiles (.profilename (Variables|Defaults|GetDefaultKeyboard)) (Variables|Defaults|GetDefaultKeyboard))
  (CallFunction|SaveUserProfiles)
  (return))

(fn DeleteProfile
  (params (ToDelete :type String))
  (bind _userprofiles (Variables|Default|GetUserProfiles))
  (if (or (Utilities|Enum|Equal(Enum) ToDelete (.profilename (Variables|Defaults|GetDefaultController))) (Utilities|Enum|Equal(Enum) ToDelete (.profilename (Variables|Defaults|GetDefaultKeyboard))))
    (bind _returnvalue (UserInterface|CreateWidget "/Game/UI/Title/SimpleDialogue.SimpleDialogue_C"))
    (bind _output_get (Variables|Default|SetDialogueBox _returnvalue))
    (Default|SetMessage _output_get "Cannot delete a default profile,")
    (UserInterface|Viewport|AddtoViewport _output_get 0)
    (else
      (Utilities|Map|Remove _userprofiles ToDelete)
      (CallFunction|SaveUserProfiles)))
  (return _userprofiles))