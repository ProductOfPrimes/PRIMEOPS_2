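; BP_ShallowWater is a water volume that slows mechs while they overlap it.
; On overlap begin, it spawns a missile-explosion Niagara effect at any entering actor, then adds a speed modifier to a Mech_Pawn's movement component.
; It stores each modifier handle in a map keyed by PlayerInt, so overlap end can remove that mech's slow.
; Both transitions print debug messages for mechs.
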(event EventBeginPlay)

(event EventTick
  (params (DeltaSeconds :type Float%20%28single-precision%29)))

(event Collision|EventActorBeginOverlap
  (params (OtherActor :type Actor%20Object%20Reference))
  (Niagara|SpawnSystematLocation "/Game/VFX/Impacts/NS_ProjectileImpact_ExplosionMissile.NS_ProjectileImpact_ExplosionMissile" (Transformation|GetActorLocation OtherActor))
  (bind _asmech_pawn (Utilities|Casting|CastToMech_Pawn OtherActor))
  (bind _id (Default|AddSpeedModifier (Variables|/Game/Blueprints/Mech_Pawn.Mech_Pawn_C|GetMechMovementComponent _asmech_pawn) (Variables|Default|GetSpeedModifierInWater)))
  (Utilities|Map|Add (Variables|Default|GetSlowEffectsApplied) (Variables|/Game/Blueprints/Mech_Pawn.Mech_Pawn_C|GetPlayerInt _asmech_pawn) _id)
  (Development|PrintString (Utilities|String|Append (Utilities|GetDisplayName _asmech_pawn) " is in water!!")))

(event Collision|EventActorEndOverlap
  (params (OtherActor :type Actor%20Object%20Reference))
  (bind _asmech_pawn (Utilities|Casting|CastToMech_Pawn OtherActor))
  (Default|RemoveSpeedModifier (Variables|/Game/Blueprints/Mech_Pawn.Mech_Pawn_C|GetMechMovementComponent _asmech_pawn) (.Value (Utilities|Map|Find (Variables|Default|GetSlowEffectsApplied) (Variables|/Game/Blueprints/Mech_Pawn.Mech_Pawn_C|GetPlayerInt _asmech_pawn))))
  (Utilities|Map|Remove (Variables|Default|GetSlowEffectsApplied) (Variables|/Game/Blueprints/Mech_Pawn.Mech_Pawn_C|GetPlayerInt _asmech_pawn))
  (Development|PrintString (Utilities|String|Append (Utilities|GetDisplayName _asmech_pawn) " is out of water!!") true true "(R=0.427083,G=0.647944,B=1.000000,A=1.000000)"))

(fn ConstructionScript
  (|CallParentFunction))